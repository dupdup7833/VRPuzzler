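; BP_Fuse2 is a hand-grabbable fuse with wrist-inventory support that can be force-pulled to a hand.
; A ghost mesh shows hover, and a spline mesh ray points toward the connected hand while Tick is enabled.
; Pull launches it along a projectile arc, while Pickup attaches it through InventoryItem and poses skeletal hands.
; Drop restores physics, or places it at the supplied transform without physics when IsFuseConnected is set.
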(event `self.ReceiveBeginPlay`
  ;[1 1 1] Get the initial scale and mesh materials used in the wrist slot
  (set `/Game/VRInventory/Blueprints/BPC_InventoryItem.InitialScale` (`SceneComponent.K2_GetComponentScale` (`self.StaticMeshComponent`)) (`self.InventoryItem`))
  (set `/Game/VRInventory/Blueprints/BPC_InventoryItem.DefaultMaterials` (`MeshComponent.GetMaterials` (`self.StaticMeshComponent`)) (`self.InventoryItem`))
  (`PrimitiveComponent.SetSimulatePhysics` (`self.StaticMeshComponent`) (`self.bSimulatePhysics?`))
  (set `/Game/VRInventory/Blueprints/BPC_InventoryItem.bSnapToSocket?` (`self.bSnapToSocket?`) (`self.InventoryItem`))
  (set `/Game/VRInventory/Blueprints/BPC_InventoryItem.SocketName` (`self.SocketName`) (`self.InventoryItem`))
  (set `/Game/VRInventory/Blueprints/BPC_InventoryItem.WristStoredScalePercentage` (`self.WristStoredScalePercentage`) (`self.InventoryItem`)))

(event `self.ReceiveTick`
  (params (DeltaSeconds :type "Float (single-precision)"))
  ;[1 1 1] Update the line that shows a connection with the hand that will pull the object
  (bind _handreference (`self.HandReference`)
    (:`then`
      (`SceneComponent.K2_SetWorldRotation` (`self.Spline`) (`self.GetSplineRotationToHand` _handreference) false false)
      (`SplineComponent.SetLocationAtSplinePoint` (`self.Spline`) 1 (`self.GetLocationBetweenHandAndPickup` _handreference) "World" true)
      (`self.UpdateSplineMesh`))
    (:`else`)))

(event `/Game/VRInventory/Blueprints/BI_GrabForcePickup.Pickup`
  (params (AttachTo :type "SceneComponent Object Reference") (Hand :type "EControllerHand Enum" :default "Left"))
  (bind _staticmeshcomponent (`self.StaticMeshComponent`))
  (bind _attachtocomp (`/Game/VRInventory/Blueprints/BPC_InventoryItem.AttachToComp` (`self.InventoryItem`)))
  ;[1 1 1] Pick up and drop the object
  (bind _output_get (set `/Game/VRInventory/Blueprints/BPC_InventoryItem.AttachToComp` AttachTo (`self.InventoryItem`)))
  (if (not (`ActorComponent.ComponentHasTag` _output_get "BusyHand"))
    (set `/Game/VRInventory/Blueprints/BPC_InventoryItem.Hand` Hand (`self.InventoryItem`))
    (if (`/Game/VRInventory/Blueprints/BPC_InventoryItem.bCanPickupItem?` (`self.InventoryItem`))
      (`/Game/VRInventory/Blueprints/BPC_InventoryItem.OnPickup` (`self.InventoryItem`))
      (set `self.bHeld` true)
      (`PrimitiveComponent.SetSimulatePhysics` (`self.StaticMeshComponent`) false)
      (if (`self.bSnapToSocket?`)
        (`SceneComponent.K2_AttachToComponent` _staticmeshcomponent _attachtocomp (`self.SocketName`) "SnapToTarget" "SnapToTarget" "KeepWorld" false)
        (else
          (`SceneComponent.K2_AttachToComponent` _staticmeshcomponent _attachtocomp "None" "KeepWorld" "KeepWorld" "KeepWorld" false)))
      (set `self.bIsPickedUp?` true)
      (`self.UpdateHandAnimPose`)
      (set `self.GotPulled` false))))

(event `/Game/VRInventory/Blueprints/BI_GrabForcePickup.Pull`
  ;[1 1 1] Called when pulling the object.
  (`self.HandReference`
    (:`then`
      (set `self.GotPulled` true)
      (`PrimitiveComponent.SetCollisionResponseToChannel` (`self.StaticMeshComponent`) "ECC_GameTraceChannel1" "ECR_Ignore")
      (`PrimitiveComponent.SetSimulatePhysics` (`self.StaticMeshComponent`) true)
      (`/Game/VRInventory/Blueprints/BI_GrabForcePickup.Disconnect`)
      (`/Game/VRInventory/Blueprints/BI_GrabForcePickup.Unhover`)
      (`PrimitiveComponent.SetSimulatePhysics` (`self.StaticMeshComponent`) false)
      (bind _outlaunchvelocity (`GameplayStatics.SuggestProjectileVelocity_CustomArc` (`SceneComponent.K2_GetComponentLocation` (`self.StaticMeshComponent`)) (`SceneComponent.K2_GetComponentLocation` (`self.HandReference`)) (`self.ObjectGravity`) (`self.ObjectPullArc`)))
      (`PrimitiveComponent.SetSimulatePhysics` (`self.StaticMeshComponent`) true)
      (`PrimitiveComponent.AddImpulse` (`self.StaticMeshComponent`) _outlaunchvelocity "None" true))
    (:`else`)))

(event `/Game/VRInventory/Blueprints/BI_GrabForcePickup.Drop`
  (params (setLocation :type "Vector Structure") (setRotation :type "Rotator Structure"))
  ;[1 1 1] On drop, drop the object and call the on release dispatcher as well as updating the picked up state
  (if (`self.isFuseConnected`)
    (`PrimitiveComponent.SetSimulatePhysics` (`self.StaticMeshComponent`) false)
    (`self.K2_DetachFromActor` "KeepWorld" "KeepWorld" "KeepWorld")
    (`self.K2_SetActorLocationAndRotation` setLocation setRotation)
    (`/Game/VRInventory/Blueprints/BPC_InventoryItem.OnRelease` (`self.InventoryItem`))
    (set `self.bIsPickedUp?` false)
    (`self.ResetHandAnimState`)
    (set `self.GotPulled` false)
    (set `self.bHeld` false)
    (else
      (`self.K2_DetachFromActor` "KeepWorld" "KeepWorld" "KeepWorld")
      (`PrimitiveComponent.SetSimulatePhysics` (`self.StaticMeshComponent`) true)
      (`/Game/VRInventory/Blueprints/BPC_InventoryItem.OnRelease` (`self.InventoryItem`))
      (set `self.bIsPickedUp?` false)
      (`self.ResetHandAnimState`)
      (set `self.GotPulled` false)
      (set `self.bHeld` false))))

(event `/Game/VRInventory/Blueprints/BI_GrabForcePickup.ConnectHand`
  (params (Hand :type "SceneComponent Object Reference"))
  ;[1 1 1] Connect and disconnect from hand
  (if (`/Game/VRInventory/Blueprints/BPC_InventoryItem.bCanPickupItem?` (`self.InventoryItem`))
    (set `self.HandReference` Hand)
    (`self.SetActorTickEnabled` true)
    (set `self.ConnectedToHand` true)))

(event `/Game/VRInventory/Blueprints/BI_GrabForcePickup.Disconnect`
  ;[1 1 1] Connect and disconnect from hand
  (if (`/Game/VRInventory/Blueprints/BPC_InventoryItem.bCanPickupItem?` (`self.InventoryItem`))
    (`self.SetActorTickEnabled` false)
    (`SplineComponent.SetLocationAtSplinePoint` (`self.Spline`) 1 (`SplineComponent.GetLocationAtSplinePoint` (`self.Spline`) 0 "World") "World" true)
    (`self.UpdateSplineMesh`)
    (set `self.ConnectedToHand` false)))

(event `self.StaticMeshComponent.OnComponentHit`
  (params (HitComponent :type "PrimitiveComponent Object Reference") (OtherActor :type "Actor Object Reference") (OtherComp :type "PrimitiveComponent Object Reference") (NormalImpulse :type "Vector Structure") (Hit :type "HitResult Structure (by ref)"))
  ;[1 1 1] Disable collision with the hand when being pulled
  (if (`self.GotPulled`)
    (set `self.GotPulled` false)
    (`PrimitiveComponent.SetCollisionResponseToChannel` (`self.StaticMeshComponent`) "ECC_GameTraceChannel1" "ECR_Block")
    (`/Game/VRInventory/Blueprints/BPC_InventoryItem.OnPickupLanding` (`self.InventoryItem`))))

(event `/Game/VRInventory/Blueprints/BI_GrabForcePickup.Hover`
  ;[1 1 1] Connect and disconnect from hand
  ;[1 1 1] Hover and Unhover
  (if (`/Game/VRInventory/Blueprints/BPC_InventoryItem.bCanPickupItem?` (`self.InventoryItem`))
    (`SceneComponent.SetHiddenInGame` (`self.GhostMesh`) false false)
    (`SceneComponent.SetVisibility` (`self.GhostMesh`) true false)))

(event `/Game/VRInventory/Blueprints/BI_GrabForcePickup.Unhover`
  ;[1 1 1] Hover and Unhover
  (if (`/Game/VRInventory/Blueprints/BPC_InventoryItem.bCanPickupItem?` (`self.InventoryItem`))
    (`SceneComponent.SetHiddenInGame` (`self.GhostMesh`) true false)
    (`SceneComponent.SetVisibility` (`self.GhostMesh`) false false)))

(fn `CanPickup?`
  (returns (Result :type Boolean))
  (bind _inventoryitem (`self.InventoryItem`))
  (return (and (`/Game/VRInventory/Blueprints/BPC_InventoryItem.bCanPickupItem?` _inventoryitem) (not (`/Game/VRInventory/Blueprints/BPC_InventoryItem.bItemStored?` _inventoryitem)))))

(fn `ConnectedToHand?`
  (returns (ReturnValue :type Boolean))
  (return (`self.ConnectedToHand`)))

(fn `GetDefaultMaterials`
  (set `self.MeshMaterials` (`MeshComponent.GetMaterials` (`self.StaticMeshComponent`)))
  (`self.UpdateMeshMaterials`))

(fn `GetHandPoses`
  (returns (LeftHandPose :type "AnimSequence Object Reference") (RightHandPose :type "AnimSequence Object Reference"))
  (return (`self.LeftGrabAnimation`) (`self.RightGrabAnimation`)))

(fn `GetLocationBetweenHandAndPickup`
  (params (SceneComponent :type "SceneComponent Object Reference"))
  (returns (ReturnValue :type "Vector Structure"))
  (bind _returnvalue (- (`SceneComponent.K2_GetComponentLocation` SceneComponent) (`SceneComponent.K2_GetComponentLocation` (`self.Spline`))))
  (return (+ (`SceneComponent.K2_GetComponentLocation` (`self.Spline`)) (* (`KismetMathLibrary.Normal` _returnvalue) (/ (`KismetMathLibrary.Abs` (`KismetMathLibrary.VSize` _returnvalue)) (`self.RayLength`))))))

(fn `GetSplineRotationToHand`
  (params (Hand :type "SceneComponent Object Reference"))
  (returns (ReturnValue :type "Rotator Structure"))
  (return (`KismetMathLibrary.FindLookAtRotation` (`SceneComponent.K2_GetComponentLocation` (`self.Spline`)) (`SceneComponent.K2_GetComponentLocation` Hand))))

(fn `Held?`
  (returns (Result :type Boolean))
  (return (`self.bHeld`)))

(fn `ResetHandAnimState`
  (bind _attachtocomp (`/Game/VRInventory/Blueprints/BPC_InventoryItem.AttachToComp` (`self.InventoryItem`))
    (:`then`
      (bind _asskeletal_mesh_component (cast `SkeletalMeshComponent` _attachtocomp))
      (`SkeletalMeshComponent.SetAnimationMode` _asskeletal_mesh_component "AnimationBlueprint"))
    (:`else`)))

(fn `UpdateHandAnimPose`
  (switch `EControllerHand` (`/Game/VRInventory/Blueprints/BPC_InventoryItem.Hand` (`self.InventoryItem`))
    (:`Left`
      (`self.LeftGrabAnimation`
        (:`then`
          _)
        (:`else`)))
    (:`Right`
      (`self.RightGrabAnimation`
        (:`then`
          _)
        (:`else`))))
  (bind _asskeletal_mesh_component (cast `SkeletalMeshComponent` (`/Game/VRInventory/Blueprints/BPC_InventoryItem.AttachToComp` (`self.InventoryItem`)))
    (:`then`
      (set `self.CachedAnimClass` (`SkeletalMeshComponent.AnimClass` _asskeletal_mesh_component))
      (set `SkeletalMeshComponent.AnimationData` (make `SingleAnimationPlayData` (select `EControllerHand` (`/Game/VRInventory/Blueprints/BPC_InventoryItem.Hand` (`self.InventoryItem`)) :`Left` (`self.LeftGrabAnimation`) :`Right` (`self.RightGrabAnimation`)) false) _asskeletal_mesh_component)
      (`SkeletalMeshComponent.SetAnimationMode` _asskeletal_mesh_component "AnimationSingleNode"))
    (:`CastFailed`
      (`KismetSystemLibrary.PrintString` "You have specified an hand pose for a wrist inventory object but the component you are passing as a parameter in the pick up interface call isn't a skeletal mesh. If you want to pose your hand correctly make sure to update the interface pick up call by passing the hand reference as the attached to parameter" true true (struct :`R` 1.0 :`A` 1.0) 10.0))))

(fn `UpdateMeshMaterials`
  (for (_ _array_index) (`MeshComponent.GetMaterials` (`self.StaticMeshComponent`))
    (if (`KismetArrayLibrary.Array_IsValidIndex` (`self.MeshMaterials`) _array_index)
      (`PrimitiveComponent.SetMaterial` (`self.StaticMeshComponent`) _array_index (`|GetArrayItem` (`self.MeshMaterials`) _array_index))
      (`PrimitiveComponent.SetMaterial` (`self.GhostMesh`) _array_index "/Game/VRInventory/Materials/MaterialInstances/MI_GhostMesh.MI_GhostMesh"))))

(fn `UpdateSplineMesh`
  (`SplineMeshComponent.SetStartAndEnd` (`self.SplineMesh`) (`SplineComponent.GetLocationAtSplinePoint` (`self.Spline`) 0 "Local") (`SplineComponent.GetTangentAtSplinePoint` (`self.Spline`) 0 "Local") (`SplineComponent.GetLocationAtSplinePoint` (`self.Spline`) 1 "Local") (`SplineComponent.GetTangentAtSplinePoint` (`self.Spline`) 1 "Local") true))

(fn `UserConstructionScript`
  (`self.UpdateSplineMesh`) ; Initially update the mesh to make it \ncollapse so that it's not visible to start with.
  (`SceneComponent.K2_AttachToComponent` (`self.Spline`) (`self.StaticMeshComponent`) "None" "KeepWorld" "KeepWorld" "KeepWorld" false) ; Attach the spline at runtime so that we keep its scale.\nIf we'd parent it in the component view then it would \nscale with the mesh. We obviously make the scale rule\nkeep world.
  ;[1 1 1] Base mesh and ghost mesh
  (`StaticMeshComponent.SetStaticMesh` (`self.StaticMeshComponent`) (`self.Mesh`))
  (`StaticMeshComponent.SetStaticMesh` (`self.GhostMesh`) (`self.Mesh`))
  ;[1 1 1] The ray that represents the intention of force grabbing the object start and end size.
  (`SplineMeshComponent.SetStartScale` (`self.SplineMesh`) (`self.HandConnectionRaySizeStart`) true)
  (`SplineMeshComponent.SetEndScale` (`self.SplineMesh`) (`self.HandConnectionRaySizeEnd`) true)
  (`SceneComponent.SetVisibility` (`self.Collision`) (`self.bShowForceGrabCollision?`) false) ; Inside the editor we may want to \nhide the force grab collision
  (`SceneComponent.SetWorldScale3D` (`self.Collision`) (+ (/ (* (`.BoxExtent` (`KismetSystemLibrary.GetComponentBounds` (`self.StaticMeshComponent`))) 2.0) 100.0) (`self.ForceGrabCollisionSize`))) ; Set the collision size for force grabbing.\nWe get the base mesh local bounds and add onto\nit so that the final force grab collision is \nbigger than the mesh itself. Makes it easier to\npoint at from a distance.
  (`self.UpdateMeshMaterials`)
  (`SceneComponent.SetVisibility` (`self.GhostMesh`) (`self.bShowHighlightEffect?`) false))