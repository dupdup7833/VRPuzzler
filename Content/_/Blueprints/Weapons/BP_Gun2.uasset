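; BP_Gun2 is a hand-held gun that spawns projectiles and displays its remaining ammo on a text component.
; Its InventoryItem component's pickup and release events toggle firing, while store and retrieve events hide or show the ammo text.
; Left and right fire inputs fire only when the gun is in the matching hand.
; Each shot decrements the ammo, instantly refills it at zero, and spawns BP_Projectile at the spawn point.
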(event `self.ReceiveBeginPlay`
  (`parent.ReceiveBeginPlay`)
  (add `/Game/VRInv/Blueprints/BPC_InventoryItem.OnPickup` (`self.InventoryItem`) (`|CreateDelegate` :!event `Pickedup`))
  (add `/Game/VRInv/Blueprints/BPC_InventoryItem.OnRelease` (`self.InventoryItem`) (`|CreateDelegate` :!event `Released`))
  (add `/Game/VRInv/Blueprints/BPC_InventoryItem.OnItemStored` (`self.InventoryItem`) (`|CreateDelegate` :!event `OnItemStored`))
  (add `/Game/VRInv/Blueprints/BPC_InventoryItem.OnItemRetrieved` (`self.InventoryItem`) (`|CreateDelegate` :!event `OnItemRetrieved`))
  (`self.EnableInput` (`GameplayStatics.GetPlayerController` 0)))

(event `OnItemStored`
  (`SceneComponent.SetHiddenInGame` (`self.AmmoText`) true false))

(event `OnItemRetrieved`
  (`SceneComponent.SetHiddenInGame` (`self.AmmoText`) false false))

(event `Pickedup`
  (set `self.bCanFire?` true))

(event `Released`
  (set `self.bCanFire?` false))

(event `InputAction|RightFire` :consume false
  (params (Key :type "Key Structure"))
  (:`Pressed`
    (if (`self.bCanFire?`)
      (switch `EControllerHand` (`/Game/VRInv/Blueprints/BPC_InventoryItem.Hand` (`self.InventoryItem`))
        (:`Right`
          (`self.Fire`))))))

(event `InputAction|LeftFire` :consume false
  (params (Key :type "Key Structure"))
  (:`Pressed`
    (if (`self.bCanFire?`)
      (switch `EControllerHand` (`/Game/VRInv/Blueprints/BPC_InventoryItem.Hand` (`self.InventoryItem`))
        (:`Left`
          (`self.Fire`))))))

(fn `Fire`
  (bind _ammo (`self.Ammo`))
  (set `self.Ammo` (- _ammo 1))
  (if (<= _ammo 0)
    (set `self.Ammo` (`self.TotalAmmo`)))
  (`TextRenderComponent.K2_SetText` (`self.AmmoText`) (`KismetTextLibrary.Conv_IntToText` _ammo))
  (`|SpawnActorFromClass` "/Game/VRInv/Blueprints/Examples/BP_Projectile.BP_Projectile_C" (`SceneComponent.K2_GetComponentToWorld` (`self.ProjectileSpawnPoint`)) "AlwaysSpawn" "OverrideRootScale" null null))

(fn `UserConstructionScript`
  (`parent.UserConstructionScript`))