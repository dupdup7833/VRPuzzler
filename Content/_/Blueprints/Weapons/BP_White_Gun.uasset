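; BP_White_Gun is a hand-held, pickup-able gun that fires projectiles and tracks its ammo.
; Pickup enables firing, and left or right fire input shoots only when it matches the holding hand.
; Each shot spawns a projectile, auto-refills empty ammo, updates text and inventory info, then runs a debug sphere trace printing the hit actor.
; Inventory interface SaveState and LoadState persist ammo in the "Gun" save slot.
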(event `self.ReceiveBeginPlay`
  ;[1 1 1] On being play bind to pickedup and enable inputs since this is an actor not a pawn
  (`parent.ReceiveBeginPlay`)
  (add `self.OnPickup` (`|CreateDelegate` :!event `PickedUp`))
  (`self.EnableInput` (`GameplayStatics.GetPlayerController` 0)))

(event `PickedUp`
  ;[1 1 1] The parent class has a picked up event dispatchers that fires this event so that we udpate the info as soon as we pick it up and enable can fire.
  (set `self.bCanFire?` true)
  (`self.UpdateGunInfo`))

(event `InputAction|RightFire` :consume false
  (params (Key :type "Key Structure"))
  ;[1 1 1] Fire the gun
  (:`Pressed`
    (if (`self.bCanFire?`)
      (switch `EControllerHand` (`self.Hand`)
        (:`Right`
          (`self.Fire`))))))

(event `InputAction|LeftFire` :consume false
  (params (Key :type "Key Structure"))
  ;[1 1 1] Fire the gun
  (:`Pressed`
    (if (`self.bCanFire?`)
      (switch `EControllerHand` (`self.Hand`)
        (:`Left`
          (`self.Fire`))))))

(event `/Game/VRInv/Blueprints/BI_InventoryItem.SaveState`
  ;[1 1 1] Save and load state of actor. This is part of the inventory item interface. Make sure to implement them if you ticked bKeepItemState? inside the inventory slot
  (bind _returnvalue (`GameplayStatics.CreateSaveGameObject` "/Game/VRInv/Blueprints/Examples/BP_GunSaveGame.BP_GunSaveGame_C"))
  (set `/Game/VRInv/Blueprints/Examples/BP_GunSaveGame.Ammo` (`self.Ammo`) _returnvalue)
  (`GameplayStatics.SaveGameToSlot` _returnvalue "Gun"))

(event `/Game/VRInv/Blueprints/BI_InventoryItem.LoadState`
  ;[1 1 1] Save and load state of actor. This is part of the inventory item interface. Make sure to implement them if you ticked bKeepItemState? inside the inventory slot
  (bind _returnvalue (`GameplayStatics.DoesSaveGameExist` "Gun"))
  (if _returnvalue
    (bind _returnvalue_2 (`GameplayStatics.LoadGameFromSlot` "Gun"))
    (bind _asbp_gun_save_game (cast `/Game/VRInv/Blueprints/Examples/BP_GunSaveGame` _returnvalue_2))
    (bind _output_get (set `self.Ammo` (`/Game/VRInv/Blueprints/Examples/BP_GunSaveGame.Ammo` _asbp_gun_save_game)))
    (`TextRenderComponent.K2_SetText` (`self.AmmoText`) (`KismetTextLibrary.Conv_IntToText` _output_get))
    (`self.UpdateGunInfo`)))

(fn `Fire`
  (bind _ammo (`self.Ammo`))
  (set `self.Ammo` (- _ammo 1))
  (if (<= _ammo 0)
    (set `self.Ammo` (`self.TotalAmmo`)))
  (`TextRenderComponent.K2_SetText` (`self.AmmoText`) (`KismetTextLibrary.Conv_IntToText` _ammo))
  (`self.UpdateGunInfo`)
  (bind _returnvalue (`|SpawnActorFromClass` (`self.ProjectileClass`) (`SceneComponent.K2_GetComponentToWorld` (`self.ProjectileSpawnPoint`)) "AlwaysSpawn" "OverrideRootScale" null null))
  (`self.ThreadTrace` _returnvalue))

(fn `ThreadTrace`
  (params (Projectile :type "Actor Object Reference"))
  (bind _arrow (`self.Arrow`))
  (bind _returnvalue (`SceneComponent.K2_GetComponentLocation` _arrow))
  (bind _outhit (`KismetSystemLibrary.SphereTraceSingle` _returnvalue (+ _returnvalue (* (`KismetMathLibrary.GetForwardVector` (`SceneComponent.K2_GetComponentRotation` _arrow)) (`self.Range`))) (`self.ThreadSize`) "TraceTypeQuery2" false (`|MakeArray` (`GameplayStatics.GetPlayerPawn` 0) Projectile :!type "Actor Object Reference") "Persistent"))
  (`KismetSystemLibrary.PrintString` (`KismetSystemLibrary.GetDisplayName` (`.HitActor` (`GameplayStatics.BreakHitResult` _outhit)))))

(fn `UpdateGunInfo`
  (`/Game/VRInv/Blueprints/BPC_InventoryItemInfo.UpdateInventoryInfo` (`self.InventoryItemInfo`) (`|FormatText` "{0}/{1}" (`KismetTextLibrary.Conv_IntToText` (`self.Ammo`)) (`KismetTextLibrary.Conv_IntToText` (`self.TotalAmmo`)))))

(fn `UserConstructionScript`
  (`parent.UserConstructionScript`))