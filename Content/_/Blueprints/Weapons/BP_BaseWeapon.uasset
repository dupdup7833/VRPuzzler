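; Base weapon Blueprint, used as a child actor, that auto-fires thunder ball projectiles while firing is active.
; StartFiring loops on a delay until StopFiring clears the flag, spawning scaled-down BP_thunderBall_Puzzler actors at the Arrow, aimed along the parent actor's forward vector.
; Separate functions spawn a BP_Projectile at the barrel and run a debug-drawn threat sphere trace along the Arrow; neither is called within this Blueprint.
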(event `Start Firing`
  (if (not (`self.isFiring`))
    (set `self.isFiring` true)
    (bind _returnvalue (`|SpawnActorFromClass` "/Game/_/Blueprints/Weapons/BP_thunderBall_Puzzler.BP_thunderBall_Puzzler_C" (`KismetMathLibrary.MakeTransform` (`SceneComponent.K2_GetComponentLocation` (`self.Arrow`)) (`KismetMathLibrary.Conv_VectorToRotator` (`KismetMathLibrary.GetForwardVector` (`self.K2_GetActorRotation` (`self.GetParentActor`))))) "AlwaysSpawn" "OverrideRootScale" null null :!label _label))
    (`SceneComponent.SetWorldScale3D` (`Actor.RootComponent` _returnvalue) (0.25 0.25 0.25))
    (`KismetSystemLibrary.Delay` (`self.FiringDelay`))
    (if (`self.isFiring`)
      (goto _label))))

(event `StopFiring`
  (set `self.isFiring` false))

(fn `FireBullet`
  (`|SpawnActorFromClass` "/Game/VRInv/Blueprints/Examples/BP_Projectile.BP_Projectile_C" (`SceneComponent.K2_GetComponentToWorld` (`self.BarrelReference`)) "Undefined" "OverrideRootScale" null null))

(fn `NewFunction_0`)

(fn `ThreatTrace`
  (bind _arrow (`self.Arrow`))
  (bind _returnvalue (`SceneComponent.K2_GetComponentLocation` _arrow))
  (`KismetSystemLibrary.SphereTraceSingle` :`Start` _returnvalue :`End` (+ _returnvalue (* (`KismetMathLibrary.GetForwardVector` (`SceneComponent.K2_GetComponentRotation` _arrow)) (`self.Range`))) :`Radius` (`self.ThreatSize`) :`TraceChannel` "TraceTypeQuery1" :`DrawDebugType` "Persistent"))

(fn `UserConstructionScript`)