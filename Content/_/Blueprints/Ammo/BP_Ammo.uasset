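; BP_Ammo is an ammo pickup that spins in place until the player walks over it.
; A timeline started on BeginPlay drives the mesh's yaw, with a fixed roll tilt.
; On box overlap, DestroyOnPickup checks the other actor through an IsPlayer interface message.
; For a player, it destroys the pickup, messages the player pawn's primary weapon to pick up ammo and prints that weapon's name.
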(event `self.ReceiveBeginPlay`
  (bind (_direction _rotationcurve) (`Timeline|RotateAmmo`)
    (:`Update`
      (`SceneComponent.K2_SetWorldRotation` (`self.AmmoMesh`) (`KismetMathLibrary.MakeRotator` 15.0 0.0 _rotationcurve) false false))))

(event `self.BoxCollision.OnComponentBeginOverlap`
  (params (OverlappedComponent :type "PrimitiveComponent Object Reference") (OtherActor :type "Actor Object Reference") (OtherComp :type "PrimitiveComponent Object Reference") (OtherBodyIndex :type Integer) (bFromSweep :type Boolean) (SweepResult :type "HitResult Structure (by ref)"))
  (`self.DestroyOnPickup` OtherActor))

(fn `UserConstructionScript`)