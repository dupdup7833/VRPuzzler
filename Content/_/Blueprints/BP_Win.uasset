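; BP_Win is a puzzle win-indicator actor whose sphere shows whether an accumulated point total matches the required amount.
; A Solve event adds the incoming amount to a running Value and compares it with PointsRequired for exact equality.
; On a match the sphere switches to a fire material, otherwise to CubeMaterial, and the new total is printed for debugging.
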(event `/Game/_/Blueprints/BPI_SolveFuseBox.Solve`
  (params (RequiredValue :type Integer))
  (bind _output_get (set `self.Value` (+ RequiredValue (`self.Value`))))
  (if (== (`self.PointsRequired`) _output_get)
    (`PrimitiveComponent.SetMaterial` (`self.Sphere`) 0 "/Game/WesterTown/Materials/Effects/M_Effects_Fire.M_Effects_Fire")
    (else
      (`PrimitiveComponent.SetMaterial` (`self.Sphere`) 0 "/Game/Geometry/Meshes/CubeMaterial.CubeMaterial")))
  (`KismetSystemLibrary.PrintString` (`KismetStringLibrary.Conv_IntToString` (`self.Value`))))

(fn `UserConstructionScript`)