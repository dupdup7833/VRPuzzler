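; Fuse box puzzle actor with three sockets, each accepting one specific fuse actor.
; When the required fuse overlaps its socket, it is flagged connected and sent a drop message with the socket's location and rotation to lock it in place.
; Each insertion sends +1 and each removal -1 via a solve message to the Activate target, which receives the running changes.
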(event `self.FuseLocation1.OnComponentBeginOverlap`
  (params (OverlappedComponent :type "PrimitiveComponent Object Reference") (OtherActor :type "Actor Object Reference") (OtherComp :type "PrimitiveComponent Object Reference") (OtherBodyIndex :type Integer) (bFromSweep :type Boolean) (SweepResult :type "HitResult Structure (by ref)"))
  (bind _fuserequired1 (`self.FuseRequired1`))
  (bind _fuselocation1 (`self.FuseLocation1`))
  ;[1 1 1] Fuse 1 Locking
  (if (== OtherActor _fuserequired1)
    (bind _asbp_fuse_2 (cast `/Game/_/Blueprints/BP_Fuse2` _fuserequired1))
    (set `/Game/_/Blueprints/BP_Fuse2.isFuseConnected` true _asbp_fuse_2)
    (message `/Game/VRInv/Blueprints/BI_GrabForcePickup.Drop` (`self.FuseRequired1`) (`SceneComponent.K2_GetComponentLocation` _fuselocation1) (`SceneComponent.K2_GetComponentRotation` _fuselocation1))
    (message `/Game/_/Blueprints/BPI_SolveFuseBox.Solve` (`self.Activate`) 1)))

(event `self.FuseLocation1.OnComponentEndOverlap`
  (params (OverlappedComponent :type "PrimitiveComponent Object Reference") (OtherActor :type "Actor Object Reference") (OtherComp :type "PrimitiveComponent Object Reference") (OtherBodyIndex :type Integer))
  (bind _fuserequired1 (`self.FuseRequired1`))
  ;[1 1 1] Fuse 1 Locking
  (if (== OtherActor _fuserequired1)
    (bind _asbp_fuse_2 (cast `/Game/_/Blueprints/BP_Fuse2` _fuserequired1))
    (set `/Game/_/Blueprints/BP_Fuse2.isFuseConnected` false _asbp_fuse_2)
    (message `/Game/_/Blueprints/BPI_SolveFuseBox.Solve` (`self.Activate`) -1)))

(event `self.FuseLocation2.OnComponentBeginOverlap`
  (params (OverlappedComponent :type "PrimitiveComponent Object Reference") (OtherActor :type "Actor Object Reference") (OtherComp :type "PrimitiveComponent Object Reference") (OtherBodyIndex :type Integer) (bFromSweep :type Boolean) (SweepResult :type "HitResult Structure (by ref)"))
  (bind _fuserequired2 (`self.FuseRequired2`))
  (bind _fuselocation2 (`self.FuseLocation2`))
  (if (== OtherActor _fuserequired2)
    (bind _asbp_fuse_2 (cast `/Game/_/Blueprints/BP_Fuse2` _fuserequired2))
    (set `/Game/_/Blueprints/BP_Fuse2.isFuseConnected` true _asbp_fuse_2)
    (message `/Game/VRInv/Blueprints/BI_GrabForcePickup.Drop` (`self.FuseRequired2`) (`SceneComponent.K2_GetComponentLocation` _fuselocation2) (`SceneComponent.K2_GetComponentRotation` _fuselocation2))
    (message `/Game/_/Blueprints/BPI_SolveFuseBox.Solve` (`self.Activate`) 1)))

(event `self.FuseLocation2.OnComponentEndOverlap`
  (params (OverlappedComponent :type "PrimitiveComponent Object Reference") (OtherActor :type "Actor Object Reference") (OtherComp :type "PrimitiveComponent Object Reference") (OtherBodyIndex :type Integer))
  (bind _fuserequired2 (`self.FuseRequired2`))
  (if (== OtherActor _fuserequired2)
    (bind _asbp_fuse_2 (cast `/Game/_/Blueprints/BP_Fuse2` _fuserequired2))
    (set `/Game/_/Blueprints/BP_Fuse2.isFuseConnected` false _asbp_fuse_2)
    (message `/Game/_/Blueprints/BPI_SolveFuseBox.Solve` (`self.Activate`) -1)))

(event `self.FuseLocation3.OnComponentBeginOverlap`
  (params (OverlappedComponent :type "PrimitiveComponent Object Reference") (OtherActor :type "Actor Object Reference") (OtherComp :type "PrimitiveComponent Object Reference") (OtherBodyIndex :type Integer) (bFromSweep :type Boolean) (SweepResult :type "HitResult Structure (by ref)"))
  (bind _fuserequired3 (`self.FuseRequired3`))
  (bind _fuselocation3 (`self.FuseLocation3`))
  (if (== OtherActor _fuserequired3)
    (bind _asbp_fuse_2 (cast `/Game/_/Blueprints/BP_Fuse2` _fuserequired3))
    (set `/Game/_/Blueprints/BP_Fuse2.isFuseConnected` true _asbp_fuse_2)
    (message `/Game/VRInv/Blueprints/BI_GrabForcePickup.Drop` (`self.FuseRequired3`) (`SceneComponent.K2_GetComponentLocation` _fuselocation3) (`SceneComponent.K2_GetComponentRotation` _fuselocation3))
    (message `/Game/_/Blueprints/BPI_SolveFuseBox.Solve` (`self.Activate`) 1)))

(event `self.FuseLocation3.OnComponentEndOverlap`
  (params (OverlappedComponent :type "PrimitiveComponent Object Reference") (OtherActor :type "Actor Object Reference") (OtherComp :type "PrimitiveComponent Object Reference") (OtherBodyIndex :type Integer))
  (bind _fuserequired3 (`self.FuseRequired3`))
  (if (== OtherActor _fuserequired3)
    (bind _asbp_fuse_2 (cast `/Game/_/Blueprints/BP_Fuse2` _fuserequired3))
    (set `/Game/_/Blueprints/BP_Fuse2.isFuseConnected` false _asbp_fuse_2)
    (message `/Game/_/Blueprints/BPI_SolveFuseBox.Solve` (`self.Activate`) -1)))

(fn `UserConstructionScript`)