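; Actor component that gives a VR player a hand-anchored inventory menu, backed by a BP_Inventory actor.
; Init spawns that actor once and immediately calls its OnDestroy; SpawnInventory later moves it to the hand, facing the owner's camera.
; DestroyInventory treats a short press as a quick switch and a longer hold as a close.
; An auto-destroy event from the inventory makes the following release a no-op.
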(event `self.ReceiveBeginPlay`
  (bind _returnvalue (`Actor.GetComponentByClass` (`self.GetOwner`) "/Script/Engine.CameraComponent"))
  ;[1 1 1] Get the owner camera which is assumed the be the VR camera
  (`/Engine/EditorBlueprintResources/StandardMacros.IsValid` _returnvalue
    (:`Is Valid`
      (set `self.Camera` _returnvalue))
    (:`Is Not Valid`
      (`KismetSystemLibrary.PrintString` "Could not get camera component of parent inside of BPC_Inventory, make sure the parent of this component has at least one camera (VR camera). If the reference keeps being invalid make sure to set it manually on begin play" true true (struct :`R` 1.0 :`A` 1.0) 10.0))))

(event `Init`
  (params (HandReference :type "SkeletalMeshComponent Object Reference") (Hand :type "EControllerHand Enum" :default "Left"))
  (set `self.HandReference` HandReference)
  (set `self.Hand` Hand)
  ;[1 1 1] Spawn the inventory
  (bind _returnvalue (`|SpawnActorFromClass` "/Game/VRInventory/Blueprints/BP_Inventory.BP_Inventory_C" (`self.GetInventoryTransform` (`self.HandReference`)) "AlwaysSpawn" "OverrideRootScale" (`self.GetOwner`) (`self.HandReference`) (`self.Camera`) (`self.InventoryRotationInterpSpeed`) (`self.InventoryLocationInterpSpeed`) (`self.AutoSelect`) (`self.AutoSelectDistance`) (`self.Hand`) null))
  (bind _output_get (set `self.Inventory` _returnvalue))
  (`/Game/VRInventory/Blueprints/BP_Inventory.OnDestroy` _output_get)
  (add `/Game/VRInventory/Blueprints/BP_Inventory.OnAutoDestroy` _output_get (`|CreateDelegate` :!event `OnInvetoryAutoDestroyed`)) ; Bind to the event on auto destroy\nAuto destruction happens when the hand\nmoves far away from the menu forcing it\nto pick up the current selected item and \nauto-destroy
)

(event `SpawnInventory`
  (`self.Camera`
    (:`then`
      (`self.Inventory`
        (:`then`
          ;[1 1 1] If the inventory exists then update its transform and unhide it
          (`Actor.K2_SetActorTransform` (`self.Inventory`) (`self.GetInventoryTransform` (`self.HandReference`)) false false)
          (`/Game/VRInventory/Blueprints/BP_Inventory.OnInventorySpawned` (`self.Inventory`)) ; Call on inventory spawned on the eventory,\nit gets used to update the currently selected\nslot to the default one.
          (set `self.PressTime` (`KismetMathLibrary.Now`)) ; We get the current press time, which is used to calculate if we should a quick switch
        )
        (:`else`)))
    (:`else`
      (`KismetSystemLibrary.PrintString` "The camera reference isn't valid inside of BPC_Inventory when calling Spawn Inventory" true true (struct :`R` 1.0 :`A` 1.0) 10.0))))

(event `DestroyInventory`
  (if (not (`self.bWasAutoDestroyed?`))
    (if (> (`KismetMathLibrary.GetMilliseconds` (- (`KismetMathLibrary.Now`) (`self.PressTime`))) (`self.QuickSwitchTimeMs`))
      ;[1 1 1] On releasing the button call on destroy and hide the actor
      (bind _inventory (`self.Inventory`)
        (:`then`
          (`/Game/VRInventory/Blueprints/BP_Inventory.OnDestroy` _inventory))
        (:`else`))
      (else
        ;[1 1 1] Call quick switch instead of on destroy
        (bind _inventory_2 (`self.Inventory`)
          (:`then`
            (`/Game/VRInventory/Blueprints/BP_Inventory.QuickSwitch` _inventory_2))
          (:`else`))))
    (else
      (set `self.bWasAutoDestroyed?` false))))

(event `OnInvetoryAutoDestroyed`
  ;[1 1 1] If the inventory auto-destroyed then we don't do anything once we release the inventory button
  (set `self.bWasAutoDestroyed?` true))

(fn `GetInventoryTransform`
  (params (HandReference :type "SceneComponent Object Reference"))
  (returns (ReturnValue :type "Transform Structure"))
  (bind _returnvalue (`SceneComponent.K2_GetComponentLocation` HandReference))
  (return (`KismetMathLibrary.MakeTransform` _returnvalue (`KismetMathLibrary.FindLookAtRotation` _returnvalue (`SceneComponent.K2_GetComponentLocation` (`self.Camera`))))))