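; BP_InventoryItem is a VR inventory item that a hand can pick up and hold.
; Initialisation sets mesh, scale, snap settings and slot, disables box collision and marks it as stored.
; Pickup attaches stored items to the hand, optionally socket-snapped; otherwise, if the hand matches the inventory component's, it enables a slot, which calls Pickup again.
; ConnectedToHand and Held always return false.
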(event `/Game/VRInventory/Blueprints/BI_InventoryItem.InitialiseSM`
  (params (Mesh :type "StaticMesh Object Reference") (`Mesh Scale` :type "Vector Structure") (`bSnapToSocket?` :type Boolean) (SocketName :type Name) (Slot :type "/Game/VRInventory/Blueprints/BP_InventorySlot Object Reference"))
  ;[1 1 1] Initialise the object as a static mesh object.
  (`StaticMeshComponent.SetStaticMesh` (`self.StaticMeshComponent`) Mesh)
  (`SceneComponent.SetWorldScale3D` (`self.StaticMeshComponent`) `Mesh Scale`)
  (set `self.bSnapToSocket?` `bSnapToSocket?`)
  (set `self.SocketName` SocketName)
  (`PrimitiveComponent.SetCollisionEnabled` (`self.Box`) "NoCollision")
  (set `self.bInInventory?` true)
  (set `self.Slot` Slot))

(event `/Game/VRInventory/Blueprints/BI_InventoryItem.SetSnapBehaviour`
  (params (`bSnapToSocket?` :type Boolean) (SocketName :type Name))
  ;[1 1 1] Update the snap bahaviour of this item
  (set `self.bSnapToSocket?` `bSnapToSocket?`)
  (set `self.SocketName` SocketName))

(event `/Game/VRInventory/Blueprints/BI_GrabForcePickup.Pickup`
  (params (AttachTo :type "SceneComponent Object Reference") (Hand :type "EControllerHand Enum" :default "Left"))
  ;[1 1 1] On pick up store the hand reference. If this item is already in the inventory then just grab it otherwise enable the slot. The slot enabling process will call pick up on this object again.
  (set `self.HandReference` AttachTo)
  (if (`self.bInInventory?`)
    (if (`self.bSnapToSocket?`)
      (`self.K2_AttachToComponent` (`self.HandReference`) (`self.SocketName`) "SnapToTarget" "SnapToTarget" "KeepWorld" false)
      (else
        (`self.K2_AttachToComponent` (`self.HandReference`) "None" "KeepWorld" "KeepWorld" "KeepWorld" false)))
    (elif (`|EnumEquality` Hand (`/Game/VRInventory/Blueprints/BPC_Inventory.Hand` (`/Game/VRInventory/Blueprints/BFL_Iventory.GetInvetoryComponent` (`self.HandReference`))))
      (set `self.bInInventory?` true)
      (`/Game/VRInventory/Blueprints/BP_Inventory.EnableSlot` (`/Game/VRInventory/Blueprints/BPC_Inventory.Inventory` (`/Game/VRInventory/Blueprints/BFL_Iventory.GetInvetoryComponent` (`self.HandReference`))) self (`StaticMeshComponent.StaticMesh` (`self.StaticMeshComponent`)) null))))

(fn `ConnectedToHand?`
  (returns (ReturnValue :type Boolean))
  (return false))

(fn `Held?`
  (returns (Result :type Boolean))
  (return false))

(fn `UserConstructionScript`
  (`BoxComponent.SetBoxExtent` (`self.Box`) (`self.CollisionExtent`) true))