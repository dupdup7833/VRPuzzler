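; BPC_InventoryItem is a VR inventory component that exposes its owning actor's mesh, which the system's slot actor needs.
; On BeginPlay it searches the owner's mesh components for one whose name contains MeshName and caches it as a static or skeletal mesh, printing a warning if MeshName is empty.
; GetMesh returns the cached mesh, preferring the static one.
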(event `self.ReceiveBeginPlay`
  (if (not (`KismetStringLibrary.IsEmpty` (`self.MeshName`)))
    (for _array_element (`Actor.K2_GetComponentsByClass` (`self.GetOwner`) "/Script/Engine.MeshComponent")
      (if (`KismetStringLibrary.Contains` (`KismetSystemLibrary.GetObjectName` _array_element) (`self.MeshName`))
        (bind _asstatic_mesh_component (cast `StaticMeshComponent` _array_element)
          (:`then`
            (set `self.StaticMeshComponent` _asstatic_mesh_component)
            (break))
          (:`CastFailed`
            (bind _asskeletal_mesh_component (cast `SkeletalMeshComponent` _array_element))
            (set `self.SkeletalMeshComponent` _asskeletal_mesh_component)
            (break)))))
    (else
      (`KismetSystemLibrary.PrintString` "Mesh name inside BPC_InvetoryItem is empty. \nCannot get the mesh of the parent actor, this is used by the  \nslot actor and it's necessary for the system to work." true true (struct :`R` 1.0 :`A` 1.0)))))

(fn `GetMesh`
  (returns (Mesh :type "MeshComponent Object Reference"))
  (bind _staticmeshcomponent (`self.StaticMeshComponent`)
    (:`then`
      (return _staticmeshcomponent))
    (:`else`
      (bind _skeletalmeshcomponent (`self.SkeletalMeshComponent`)
        (:`then`
          (return _skeletalmeshcomponent))
        (:`else`)))))