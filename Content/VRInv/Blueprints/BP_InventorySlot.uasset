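; VR inventory slot actor that previews an item mesh, highlights when a controller overlaps it, and spawns that item into the player's hand.
; Construction applies the static or skeletal preview with a slot material, while sphere overlaps drive the ring, material glow and collide dispatchers.
; Spawned items are initialised through messages, can restore saved state and update slot text via BPC_InventoryItemInfo.
; Socket-snapped items also apply a hand pose.
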(event `self.ReceiveBeginPlay`
  ;[1 1 1] On begin play create the dynamic material for the hover effect
  (bind _returnvalue (`PrimitiveComponent.CreateDynamicMaterialInstance` (`self.SlotMesh`) 0 "/Game/VRInv/Materials/MaterialInstances/MI_InventorySlot.MI_InventorySlot" "None"))
  (set `self.DM` _returnvalue)
  (if (not (`self.bIsEnabled?`))
    (`self.SetActorHiddenInGame` true)))

(event `self.Sphere.OnComponentBeginOverlap`
  (params (OverlappedComponent :type "PrimitiveComponent Object Reference") (OtherActor :type "Actor Object Reference") (OtherComp :type "PrimitiveComponent Object Reference") (OtherBodyIndex :type Integer) (bFromSweep :type Boolean) (SweepResult :type "HitResult Structure (by ref)"))
  ;[1 1 1] On collide update the inventory mesh to spawn and spawn scale by calling on controller collide event dispatcher
  (`self.ProcessOverlap` OtherComp))

(event `self.Sphere.OnComponentEndOverlap`
  (params (OverlappedComponent :type "PrimitiveComponent Object Reference") (OtherActor :type "Actor Object Reference") (OtherComp :type "PrimitiveComponent Object Reference") (OtherBodyIndex :type Integer))
  ;[1 1 1] On end overlap unhover the slot
  (if (`ActorComponent.ComponentHasTag` OtherComp "InventoryInteraction")
    (`self.OnControllerEndCollide`)
    (`SceneComponent.SetHiddenInGame` (`self.Ring`) true false)
    (`MaterialInstanceDynamic.SetScalarParameterValue` (`self.DM`) "ColourIncrease" 1.0)))

(event `SpawnMesh`
  (params (HandReference :type "SkeletalMeshComponent Object Reference"))
  ;[1 1 1] Spawn and destroy/hide mesh
  (if (not (`self.bIsHand?`))
    (`self.SpawnItem` HandReference)
    (`self.ForceCheckOverlap`)
    (`self.UpdateHandPose` HandReference)
    (else
      (`SkeletalMeshComponent.SetAnimationMode` HandReference "AnimationBlueprint"))))

(event `DestroyItem`
  (params (Hand :type "PrimitiveComponent Object Reference"))
  ;[1 1 1] Spawn and destroy/hide mesh
  (`KismetArrayLibrary.Array_RemoveItem` (`ActorComponent.ComponentTags` Hand) "BusyHand")
  (bind _itemspawned (`self.ItemSpawned`)
    (:`then`
      (if (`self.bKeepItemState?`)
        (message `/Game/VRInv/Blueprints/BI_InventoryItem.SaveState` _itemspawned))
      (`self.K2_DestroyActor` _itemspawned))
    (:`else`)))

(event `EnableSlot`
  (params (ItemSpawned :type "Actor Object Reference") (HandReference :type "SkeletalMeshComponent Object Reference"))
  ;[1 1 1] Enable the slot
  (set `self.bIsEnabled?` true)
  (bind _output_get (set `self.ItemSpawned` ItemSpawned))
  (`self.BindToUpdateInfo` _output_get)
  (message `/Game/VRInv/Blueprints/BI_InventoryItem.SetSnapBehaviour` (`self.ItemSpawned`) (`self.SnapToSocket`) (`self.SocketName`))
  (message `/Game/VRInv/Blueprints/BI_GrabForcePickup.Pickup` (`self.ItemSpawned`) HandReference (`self.Hand`))
  (`KismetArrayLibrary.Array_Add` (`ActorComponent.ComponentTags` HandReference) "BusyHand")
  (`self.UpdateHandPose` HandReference)
  (`self.OnEnabled` self))

(event `UpdateInfo`
  (params (Info :type Text))
  ;[1 1 1] Update the info of this slot, this is called through an event dispatcher set inside Spawnitem
  (`TextRenderComponent.K2_SetText` (`self.TextRender`) Info))

(fn `BindToUpdateInfo`
  (params (Actor :type "Actor Object Reference"))
  (bind _returnvalue (`self.GetComponentByClass` Actor "/Game/VRInv/Blueprints/BPC_InventoryItemInfo.BPC_InventoryItemInfo_C"))
  (`/Engine/EditorBlueprintResources/StandardMacros.IsValid` _returnvalue
    (:`Is Valid`
      (add `/Game/VRInv/Blueprints/BPC_InventoryItemInfo.UpdateInventoryInfo` _returnvalue (`|CreateDelegate` :!event `UpdateInfo`)))))

(fn `ForceCheckOverlap`
  (bind _sphere (`self.Sphere`))
  (bind _outcomponents (`KismetSystemLibrary.ComponentOverlapComponents` _sphere (`SceneComponent.K2_GetComponentToWorld` _sphere) (`|MakeArray` "ObjectTypeQuery2" :!type "EObjectTypeQuery Enum")))
  (for _array_element _outcomponents
    (`self.ProcessOverlap` _array_element)))

(fn `GetUpdateInfoEvent`
  (params (Event :type "Delegate (by ref)"))
  (add `self.OnControllerCollide` Event)
  (return))

(fn `ProcessOverlap`
  (params (OtherComp :type "PrimitiveComponent Object Reference"))
  (if (`ActorComponent.ComponentHasTag` OtherComp "InventoryInteraction")
    (`self.OnControllerCollide` self)
    (`SceneComponent.SetHiddenInGame` (`self.Ring`) false false)
    (`MaterialInstanceDynamic.SetScalarParameterValue` (`self.DM`) "ColourIncrease" 1.2)))

(fn `SpawnItem`
  (params (HandReference :type "SkeletalMeshComponent Object Reference"))
  (bind _itemspawned (`self.ItemSpawned`))
  (if (not (`KismetSystemLibrary.IsValidClass` (`self.ItemClass`)))
    (`self.GetMeshType`
      (:`Static`
        (bind _returnvalue (`|SpawnActorFromClass` "/Game/VRInv/Blueprints/BP_InventoryItem.BP_InventoryItem_C" (`SceneComponent.K2_GetComponentToWorld` (`local.HandReference`)) "AlwaysSpawn" "OverrideRootScale" null null))
        (set `self.ItemSpawned` _returnvalue))
      (:`Skeletal`
        (bind _returnvalue_2 (`|SpawnActorFromClass` "/Game/VRInv/Blueprints/BP_SKInventoryItem.BP_SKInventoryItem_C" (`SceneComponent.K2_GetComponentToWorld` (`local.HandReference`)) "AlwaysSpawn" "OverrideRootScale" null null))
        (set `self.ItemSpawned` _returnvalue_2)))
    (else
      (bind _returnvalue_3 (`|SpawnActorFromClass` (`self.ItemClass`) (`SceneComponent.K2_GetComponentToWorld` (`local.HandReference`)) "AlwaysSpawn" "OverrideRootScale" null null))
      (set `self.ItemSpawned` _returnvalue_3)))
  (`self.GetMeshType`
    (:`Static`
      (message `/Game/VRInv/Blueprints/BI_InventoryItem.InitialiseSM` (`self.ItemSpawned`) (`self.ItemMeshSM`) (`self.MeshSpawnScale`) (`self.SnapToSocket`) (`self.SocketName`) self))
    (:`Skeletal`
      (message `/Game/VRInv/Blueprints/BI_InventoryItem.InitialiseSK` (`self.ItemSpawned`) (`self.ItemMeshSK`) (`self.MeshSpawnScale`) (`self.SnapToSocket`) (`self.SocketName`) self)))
  (message `/Game/VRInv/Blueprints/BI_GrabForcePickup.Pickup` (`self.ItemSpawned`) (`local.HandReference`) (`self.Hand`))
  (`KismetArrayLibrary.Array_Add` (`ActorComponent.ComponentTags` (`local.HandReference`)) "BusyHand")
  (bind _asbp_inventory_item (cast `/Game/VRInv/Blueprints/BP_InventoryItem` (`self.ItemSpawned`))
    (:`then`
      (`self.BindToUpdateInfo` _asbp_inventory_item))
    (:`CastFailed`
      (bind _asbp_skinventory_item (cast `/Game/VRInv/Blueprints/BP_SKInventoryItem` (`self.ItemSpawned`))
        (:`then`
          (`self.BindToUpdateInfo` _asbp_skinventory_item))
        (:`CastFailed`
          _))))
  (if (`self.bKeepItemState?`)
    (message `/Game/VRInv/Blueprints/BI_InventoryItem.LoadState` _itemspawned)
    (if (`self.ActorHasTag` _itemspawned "Weapon")
      (bind _asbp_nm_vrpawn (cast `/Game/_/Blueprints/BP_NM_VRPawn` (`GameplayStatics.GetPlayerPawn` 0)))
      (set `/Game/_/Blueprints/BP_NM_VRPawn.EquipedWeapon` (`self.ItemSpawned`) _asbp_nm_vrpawn))))

(fn `UpdateHandPose`
  (params (Hand :type "SkeletalMeshComponent Object Reference"))
  (if (`self.SnapToSocket`)
    (`SkeletalMeshComponent.SetAnimationMode` Hand "AnimationBlueprint")
    (set `SkeletalMeshComponent.AnimationData` (make `SingleAnimationPlayData` (`self.HandPose`) false) Hand)
    (`SkeletalMeshComponent.SetAnimationMode` Hand "AnimationSingleNode")))

(fn `UpdateMesh`
  (`self.GetMeshType`
    (:`Static`
      (`StaticMeshComponent.SetStaticMesh` (`self.ItemSM`) (`self.ItemMeshSM`))
      (`SceneComponent.SetWorldScale3D` (`self.ItemSM`) (`self.SlotMeshScale`))
      (`SceneComponent.K2_SetRelativeRotation` (`self.ItemSM`) (`self.SlotMeshRotation`) false false)
      (`SceneComponent.K2_SetRelativeLocation` (`self.ItemSM`) (`self.SlotMeshLocation`) false false)
      (`self.ItemSK`
        (:`then`
          (`ActorComponent.K2_DestroyComponent` (`self.ItemSK`)))
        (:`else`
          _))
      (for (_ _array_index) (`MeshComponent.GetMaterials` (`self.ItemSM`))
        (`PrimitiveComponent.SetMaterial` (`self.ItemSM`) _array_index "/Game/VRInv/Materials/M_ItemSlot.M_ItemSlot")))
    (:`Skeletal`
      (`SkinnedMeshComponent.SetSkinnedAssetAndUpdate` (`self.ItemSK`) (`self.ItemMeshSK`) true)
      (`SceneComponent.SetWorldScale3D` (`self.ItemSK`) (`self.SlotMeshScale`))
      (`SceneComponent.K2_SetRelativeRotation` (`self.ItemSK`) (`self.SlotMeshRotation`) false false)
      (`SceneComponent.K2_SetRelativeLocation` (`self.ItemSK`) (`self.SlotMeshLocation`) false false)
      (`self.ItemSM`
        (:`then`
          (`ActorComponent.K2_DestroyComponent` (`self.ItemSM`)))
        (:`else`
          _))
      (for (_ _array_index_2) (`MeshComponent.GetMaterials` (`self.ItemSK`))
        (`PrimitiveComponent.SetMaterial` (`self.ItemSK`) _array_index_2 "/Game/VRInv/Materials/M_ItemSlot.M_ItemSlot")))))

(fn `UserConstructionScript`
  (`self.UpdateMesh`))