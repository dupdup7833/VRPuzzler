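; VR hand inventory actor that shows child-actor slots, smoothly following the hand while turning toward the camera.
; Slots report controller collisions to set the selection, with the hand slot as default.
; Closing, manually or automatically when the hand moves too far if AutoSelect is on, spawns the selected item in the hand.
; QuickSwitch toggles the last selected item using the hand's BusyHand tag, and EnableSlot unlocks slots by matching mesh.
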(event `OnEnableSlot`
  (params (Slot :type "/Game/VRInv/Blueprints/BP_InventorySlot Object Reference"))
  ;[1 1 1] Go through all the child actors, check if any is an inventory slot and bind the on controller collide event
  ; Also go through all the slots and get the default one (the hand)
  (add `/Game/VRInv/Blueprints/BP_InventorySlot.OnControllerCollide` Slot (`|CreateDelegate` :!event `OnControllerCollide`))
  (set `self.LastSelectedSlot` Slot))

(event `self.ReceiveBeginPlay`
  ;[1 1 1] Go through all the child actors, check if any is an inventory slot and bind the on controller collide event
  ; Also go through all the slots and get the default one (the hand)
  (`self.GetDefaultSlotBindOnCollide`))

(event `OnControllerCollide`
  (params (InventorySlot :type "/Game/VRInv/Blueprints/BP_InventorySlot Object Reference"))
  ;[1 1 1] On controller collide is called by the single item slots event dispatchers
  (set `self.SelectedSlot` InventorySlot))

(event `self.ReceiveTick`
  (params (DeltaSeconds :type "Float (single-precision)"))
  ;[1 1 1] Update the rotaion of the Inventory to always point towards the VR camera, update the location to slowly follow the hand. Check if the controller is far from the inventory and if it is close the inventory.
  (`self.K2_SetActorRotation` (`KismetMathLibrary.RInterpTo` (`self.K2_GetActorRotation`) (`KismetMathLibrary.FindLookAtRotation` (`self.K2_GetActorLocation`) (`SceneComponent.K2_GetComponentLocation` (`self.CameraReference`))) (`GameplayStatics.GetWorldDeltaSeconds`) (`self.InventoryRotationInterpSpeed`)))
  (`self.K2_SetActorLocation` (`KismetMathLibrary.VInterpTo` (`self.K2_GetActorLocation`) (`SceneComponent.K2_GetComponentLocation` (`self.HandReference`)) (`GameplayStatics.GetWorldDeltaSeconds`) (`self.InventoryLocationInterpSpeed`)))
  (if (`self.AutoSelect`)
    (if (> (`KismetMathLibrary.Abs` (`KismetMathLibrary.VSize` (- (`self.K2_GetActorLocation`) (`SceneComponent.K2_GetComponentLocation` (`self.HandReference`))))) (`self.AutoSelectDistance`))
      (`self.OnDestroy`)
      (`self.OnAutoDestroy`)
      (bind _slot (`self.ForEachSlot`)
        (:`LoopBody`
          (`self.SetActorHiddenInGame` _slot true))))))

(event `OnDestroy`
  (bind _selectedslot (`self.SelectedSlot`))
  ;[1 1 1] On destroy is called by the pawn closing the inventory but also by this actor if the controller gets to far from it. It destroys the previous actor instance and spawns a new one
  (bind _slot (`self.ForEachSlot`)
    (:`LoopBody`
      (`/Game/VRInv/Blueprints/BP_InventorySlot.DestroyItem` _slot (`self.HandReference`))
      (`self.SetActorHiddenInGame` _slot true))
    (:`Completed`
      (`self.SetActorTickEnabled` false)
      (bind _selectedslot_2 (`self.SelectedSlot`)
        (:`then`
          (`/Game/VRInv/Blueprints/BP_InventorySlot.SpawnMesh` _selectedslot_2 (`self.HandReference`))
          (if (!= _selectedslot (`self.DefaultSlot`))
            (set `self.LastSelectedSlot` _selectedslot)))
        (:`else`)))))

(event `OnInventorySpawned`
  ;[1 1 1] Called when the inventory is spawned by the BPC_Inventory comp
  ; We enable the actor tick and make sure that the default slot is the hand slot
  (`self.SetActorTickEnabled` true)
  (set `self.SelectedSlot` (`self.DefaultSlot`))
  (bind _slot (`self.ForEachSlot`)
    (:`LoopBody`
      (if (`/Game/VRInv/Blueprints/BP_InventorySlot.bIsEnabled?` _slot)
        (`self.SetActorHiddenInGame` _slot false)))))

(event `QuickSwitch`
  (bind _handreference (`self.HandReference`))
  ;[1 1 1] This performs the quick switch when you press and release the button fast enough
  (`self.LastSelectedSlot`
    (:`then`
      (if (`ActorComponent.ComponentHasTag` (`self.HandReference`) "BusyHand")
        (`/Game/VRInv/Blueprints/BP_InventorySlot.DestroyItem` (`self.LastSelectedSlot`) _handreference)
        (`SkeletalMeshComponent.SetAnimationMode` _handreference "AnimationBlueprint")
        (else
          (`/Game/VRInv/Blueprints/BP_InventorySlot.SpawnMesh` (`self.LastSelectedSlot`) (`self.HandReference`))
          (`self.SetActorTickEnabled` false))))
    (:`else`
      _))
  (bind _slot (`self.ForEachSlot`)
    (:`LoopBody`
      (`self.SetActorHiddenInGame` _slot true))
    (:`Completed`
      (`self.SetActorTickEnabled` false))))

(fn `EnableSlot`
  (params (Item :type "Actor Object Reference") (SM :type "StaticMesh Object Reference") (SK :type "SkeletalMesh Object Reference"))
  (bind _slot (`self.ForEachSlot`)
    (:`LoopBody`
      (bind _sm (`local.SM`)
        (:`then`
          (if (== _sm (`/Game/VRInv/Blueprints/BP_InventorySlot.ItemMeshSM` _slot))
            (`/Game/VRInv/Blueprints/BP_InventorySlot.EnableSlot` _slot (`local.Item`) (`self.HandReference`) :!label _label)))
        (:`else`
          (bind _sk (`local.SK`)
            (:`then`
              (if (== _sk (`/Game/VRInv/Blueprints/BP_InventorySlot.ItemMeshSK` _slot))
                (goto _label)))
            (:`else`)))))))

(fn `GetDefaultSlotBindOnCollide`
  (bind _slot (`self.ForEachSlot`)
    (:`LoopBody`
      (set `/Game/VRInv/Blueprints/BP_InventorySlot.Hand` (`self.Hand`) _slot)
      (if (`/Game/VRInv/Blueprints/BP_InventorySlot.bIsEnabled?` _slot)
        (add `/Game/VRInv/Blueprints/BP_InventorySlot.OnControllerCollide` _slot (`|CreateDelegate` :!event `OnControllerCollide`))
        (else
          (add `/Game/VRInv/Blueprints/BP_InventorySlot.OnEnabled` _slot (`|CreateDelegate` :!event `OnEnableSlot`))))
      (if (`/Game/VRInv/Blueprints/BP_InventorySlot.bIsHand?` _slot)
        (set `self.DefaultSlot` _slot)))))

(fn `UserConstructionScript`
  (bind _slot (`self.ForEachSlot`)
    (:`LoopBody`
      (`/Game/VRInv/Blueprints/BP_InventorySlot.UpdateMesh` _slot))))