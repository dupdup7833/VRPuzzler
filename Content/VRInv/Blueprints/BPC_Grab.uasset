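; VR hand component that handles grabbing, releasing and force-pulling of objects implementing BI_GrabForcePickup.
; A line trace from the hand hovers distant pickups, and gripping connects one so a hand-velocity flick above a threshold pulls it.
; Grab attaches a pulled object caught near the hand or the nearest overlapping one, applying its hand pose.
; Release drops it only if still held by a hand, then restores the animation blueprint.
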(event `Init`
  (params (HandMesh :type "SkeletalMeshComponent Object Reference") (Hand :type "EControllerHand Enum" :default "Left") (LineTraceStartPoint :type "SceneComponent Object Reference") (GrabCollision :type "PrimitiveComponent Object Reference"))
  ;[1 1 1] Initialise the component
  (set `self.HandMesh` HandMesh)
  (set `self.HandAnimClass` (`SkeletalMeshComponent.AnimClass` HandMesh))
  (set `self.Hand` Hand)
  (set `self.LineTraceDirection` LineTraceStartPoint)
  (set `self.GrabCollision` GrabCollision))

(event `Customise`
  (params (ForceGrabMaxDistance :type "Float (double-precision)") (HandFlickVelocity :type "Float (double-precision)") (MidAirGrabDistance :type "Float (double-precision)") (HandForwardDirection :type "ESplineMeshAxis Enum" :default "X") (Debug :type Boolean))
  ;[1 1 1] Customise the component
  (set `self.ForceGrabMaxDistance` ForceGrabMaxDistance)
  (set `self.HandFlickVelocity` HandFlickVelocity)
  (set `self.MidAirGrabDistance` MidAirGrabDistance)
  (set `self.HandForwardDirection` HandForwardDirection)
  (set `self.Debug` Debug))

(event `ProcessForcePullObject`
  ;[1 1 1] Process the whole force pull machanic
  (if (`self.bEnableForceGrab?`)
    (`|ExecutionSequence`
      (:`then_0`
        (`self.DetectForcePullObject` (`self.HandMesh`) (`self.GrabCollision`)))
      (:`then_1`
        (`/Engine/EditorBlueprintResources/StandardMacros.Gate` true :!label _label
          (:`Exit`
            (`self.ProcessHandFlick` (`self.HandMesh`))))))))

(event `StartProcessHandFlick`
  ;[1 1 1] Process the whole force pull machanic
  (goto _label :!via `Open`))

(event `StopProcessHandFlick`
  ;[1 1 1] Process the whole force pull machanic
  (goto _label :!via `Close`))

(event `OnPickupLanding`
  ;[1 1 1] When the pick up has landed somewhere make sure to mark the object has pulled. Bond inside process hand flick.
  (set `self.Pulled` false))

(fn `CanForcePullObject?`
  (params (HitActor :type "Actor Object Reference") (GrabSphere :type "PrimitiveComponent Object Reference"))
  (returns (`Return Value` :type Boolean))
  (bind _result (message `/Game/VRInv/Blueprints/BI_GrabForcePickup.Held?` HitActor))
  (bind _result_2 (message `/Game/VRInv/Blueprints/BI_GrabForcePickup.CanPickup?` HitActor))
  (return (and (not _result) (`KismetSystemLibrary.DoesImplementInterface` HitActor "/Game/VRInv/Blueprints/BI_GrabForcePickup.BI_GrabForcePickup_C") (!= HitActor (`self.AttachedActor`)) (not (`PrimitiveComponent.IsOverlappingActor` GrabSphere HitActor)) _result_2)))

(fn `DetectForcePullObject`
  (params (HandMesh :type "SceneComponent Object Reference") (GrabCollision :type "PrimitiveComponent Object Reference"))
  (bind _returnvalue (`SceneComponent.K2_GetComponentLocation` (`self.LineTraceDirection`)))
  (bind _returnvalue_2 (`SceneComponent.K2_GetComponentRotation` (`self.LineTraceDirection`)))
  (if (and (== (`KismetArrayLibrary.Array_Length` (`self.GetOverlappingActors`)) 0) (== (`self.AttachedActor`) null) (not (`self.ComponentHasTag` HandMesh "BusyHand")))
    (bind (_outhit _returnvalue_3) (`KismetSystemLibrary.LineTraceSingle` _returnvalue (+ _returnvalue (* (select `ESplineMeshAxis` (`self.HandForwardDirection`) :`X` (`KismetMathLibrary.GetForwardVector` _returnvalue_2) :`Y` (`KismetMathLibrary.GetRightVector` _returnvalue_2) :`Z` (`KismetMathLibrary.GetUpVector` _returnvalue_2)) (`self.ForceGrabMaxDistance`))) "TraceTypeQuery1" true (`|MakeArray` (`self.GetOwner`)) (select `bool` (`self.Debug`) :`true` "ForOneFrame" :!type "EDrawDebugTrace Enum")))
    (if _returnvalue_3
      (bind (_bblockinghit _binitialoverlap _time _distance _location _impactpoint _normal _impactnormal _physmat _hitactor) (`GameplayStatics.BreakHitResult` _outhit))
      (if (`self.CanForcePullObject?` _hitactor (`local.GrabCollision`))
        (message `/Game/VRInv/Blueprints/BI_GrabForcePickup.Hover` _hitactor)
        (if (`self.bWantsToGrip`)
          (message `/Game/VRInv/Blueprints/BI_GrabForcePickup.ConnectHand` _hitactor (`local.HandMesh`))
          (`self.StartProcessHandFlick`))
        (bind _pickupobj (`self.PickupObj`)
          (:`then`
            (if (not (== _pickupobj _hitactor))
              (message `/Game/VRInv/Blueprints/BI_GrabForcePickup.Unhover` (`self.PickupObj`))
              (message `/Game/VRInv/Blueprints/BI_GrabForcePickup.Disconnect` (`self.PickupObj`))
              (bind _output_get (set `self.PickupObj` _hitactor :!label _label))
              (set `self.PulledObj` _output_get)))
          (:`else`
            (goto _label)))
        (else
          (bind _pickupobj_2 (`self.PickupObj` :!label _label_2)
            (:`then`
              (bind _returnvalue_4 (message `/Game/VRInv/Blueprints/BI_GrabForcePickup.ConnectedToHand?` _pickupobj_2))
              (if (not (and _returnvalue_4 (== (`self.AttachedActor`) null)))
                (message `/Game/VRInv/Blueprints/BI_GrabForcePickup.Unhover` _pickupobj_2)
                (message `/Game/VRInv/Blueprints/BI_GrabForcePickup.Disconnect` _pickupobj_2)
                (set `self.PickupObj` null)))
            (:`else`))))
      (else
        (goto _label_2)))
    (else
      (goto _label_2))))

(fn `GetActorNearHand`
  (params (GrabCollision :type "PrimitiveComponent Object Reference"))
  (returns (NearestMesh :type "Actor Object Reference"))
  (locals (NearestOverlappingActor :type "Actor Object Reference") (NearestOverlap :type "Float (double-precision)" :default 10000.0))
  (for _array_element (`PrimitiveComponent.GetOverlappingActors` GrabCollision "/Script/Engine.Actor")
    (if (`KismetSystemLibrary.DoesImplementInterface` _array_element "/Game/VRInv/Blueprints/BI_GrabForcePickup.BI_GrabForcePickup_C")
      (bind _returnvalue (`KismetMathLibrary.VSize` (- (`Actor.K2_GetActorLocation` _array_element) (`SceneComponent.K2_GetComponentLocation` GrabCollision))))
      (if (< _returnvalue (`local.NearestOverlap`))
        (set `local.NearestOverlappingActor` _array_element)
        (set `local.NearestOverlap` _returnvalue))))
  (return (`local.NearestOverlappingActor`)))

(fn `GetOverlappingActors`
  (returns (ReturnValue :type "Array of Actor Object Reference"))
  (locals (Actors :type "Array of Actor Object Reference"))
  (for _array_element (`PrimitiveComponent.GetOverlappingActors` (`self.GrabCollision`) "/Script/Engine.Actor")
    (if (`KismetSystemLibrary.DoesImplementInterface` _array_element "/Game/VRInv/Blueprints/BI_GrabForcePickup.BI_GrabForcePickup_C")
      (`KismetArrayLibrary.Array_Add` (`local.Actors`) _array_element)))
  (return (`local.Actors`)))

(fn `Grab`
  (set `self.bWantsToGrip` true)
  (if (`self.Pulled`)
    (`self.PulledObj`
      (:`then`
        (if (< (`KismetMathLibrary.Abs` (`KismetMathLibrary.VSize` (- (`SceneComponent.K2_GetComponentLocation` (`self.HandMesh`)) (`Actor.K2_GetActorLocation` (`self.PulledObj`))))) (`self.MidAirGrabDistance`))
          (set `self.AttachedActor` (`self.PulledObj`))
          (set `self.Pulled` false)
          (message `/Game/VRInv/Blueprints/BI_GrabForcePickup.Pickup` (stale _output_get) (`self.HandMesh`) (`self.Hand`) :!label _label)
          (if (not (`self.ComponentHasTag` (`self.HandMesh`) "BusyHand"))
            (bind (_lefthandpose _righthandpose) (message `/Game/VRInv/Blueprints/BI_GrabForcePickup.GetHandPoses` (`self.AttachedActor`)))
            (bind _returnvalue (select `EControllerHand` (`self.Hand`) :`Left` _lefthandpose :`Right` _righthandpose))
            (`/Engine/EditorBlueprintResources/StandardMacros.IsValid` _returnvalue
              (:`Is Valid`
                (set `SkeletalMeshComponent.AnimationData` (make `SingleAnimationPlayData` _returnvalue) (`self.HandMesh`))
                (`SkeletalMeshComponent.SetAnimationMode` (`self.HandMesh`) "AnimationSingleNode"))))))
      (:`else`
        (if (`self.Debug`)
          (`KismetSystemLibrary.PrintString` "Pulled object isn't valid inside the grab function of the BPC_ForceGrab component"))))
    (else
      (`self.PickupObj`
        (:`then`
          (`self.StartProcessHandFlick`)
          (message `/Game/VRInv/Blueprints/BI_GrabForcePickup.ConnectHand` (`self.PickupObj`) (`self.HandMesh`)))
        (:`else`
          (bind _nearestmesh (`self.GetActorNearHand` (`self.GrabCollision`)))
          (`/Engine/EditorBlueprintResources/StandardMacros.IsValid` _nearestmesh
            (:`Is Valid`
              (bind _output_get (set `self.AttachedActor` _nearestmesh))
              (goto _label))))))))

(fn `ProcessHandFlick`
  (params (HandMesh :type "PrimitiveComponent Object Reference"))
  (bind _returnvalue (`Actor.GetComponentByClass` (`self.PickupObj`) "/Game/VRInv/Blueprints/BPC_InventoryItem.BPC_InventoryItem_C"))
  (`self.PickupObj`
    (:`then`
      (bind _returnvalue_2 (`PrimitiveComponent.GetPhysicsLinearVelocity` (`local.HandMesh`) "None"))
      (if (`self.Debug`)
        (bind _returnvalue_3 (`KismetMathLibrary.Abs` (`KismetMathLibrary.VSize` _returnvalue_2)))
        (`KismetSystemLibrary.PrintString` (`KismetStringLibrary.Concat_StrStr` "Hand Velocity: " (`KismetStringLibrary.Conv_DoubleToString` _returnvalue_3))))
      (if (> _returnvalue_3 (`self.HandFlickVelocity`))
        (message `/Game/VRInv/Blueprints/BI_GrabForcePickup.Pull` (`self.PickupObj`))
        (set `self.PulledObj` (`self.PickupObj`))
        (set `self.Pulled` true)
        (`/Engine/EditorBlueprintResources/StandardMacros.IsValid` _returnvalue
          (:`Is Valid`
            (add `/Game/VRInv/Blueprints/BPC_InventoryItem.OnPickupLanding` _returnvalue (`|CreateDelegate` :!event `OnPickupLanding`)))
          (:`Is Not Valid`
            _))
        (`self.StopProcessHandFlick`)))
    (:`else`
      (`self.StopProcessHandFlick`))))

(fn `Release`
  (set `self.bWantsToGrip` false)
  (bind _pickupobj (`self.PickupObj`)
    (:`then`
      (message `/Game/VRInv/Blueprints/BI_GrabForcePickup.Unhover` _pickupobj)
      (message `/Game/VRInv/Blueprints/BI_GrabForcePickup.Disconnect` _pickupobj))
    (:`else`
      (`/Engine/EditorBlueprintResources/StandardMacros.IsValid` (`self.AttachedActor`)
        (:`Is Valid`
          (if (`self.ShouldRelease?` (`self.HandMesh`))
            (message `/Game/VRInv/Blueprints/BI_GrabForcePickup.Drop` (`self.AttachedActor`) (0.0 0.0 0.0) (struct)))
          (set `self.AttachedActor` null) ; Clear the reference
          (if (not (`self.ComponentHasTag` (`self.HandMesh`) "BusyHand"))
            (`SkeletalMeshComponent.SetAnimationMode` (`self.HandMesh`) "AnimationBlueprint")
            (`SkeletalMeshComponent.SetAnimInstanceClass` (`self.HandMesh`) (`self.HandAnimClass`))))))))

(fn `ShouldRelease?`
  (params (HandMesh :type "SkeletalMeshComponent Object Reference"))
  (returns (ReturnValue :type Boolean))
  (bind _returnvalue (`Actor.GetAttachParentActor` (`self.AttachedActor`)))
  (`self.AttachedActor`
    (:`then`
      (for _array_element (`Actor.K2_GetComponentsByClass` (`self.AttachedActor`) "/Script/Engine.SceneComponent")
        (if (== (`SceneComponent.GetAttachParent` _array_element) HandMesh)
          (return true)))
      (if (`KismetSystemLibrary.DoesImplementInterface` (`self.AttachedActor`) "/Game/VRInv/Blueprints/BI_InventoryItem.BI_InventoryItem_C")
        (`/Engine/EditorBlueprintResources/StandardMacros.IsValid` _returnvalue
          (:`Is Valid`
            (`/Engine/EditorBlueprintResources/StandardMacros.IsValid` (`Actor.GetComponentByClass` _returnvalue "BPC_Grab_C")
              (:`Is Valid`
                (return true))
              (:`Is Not Valid`
                _)))
          (:`Is Not Valid`
            _)))
      (return false))
    (:`else`
      (return false))))