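; VR wrist inventory slot, a child of a base slot class, that presents stored items and reacts to hand and item overlaps.
; Each tick it turns the item anchor toward the inventory's attach socket when tracking the hand, otherwise toward the camera, and updates item transforms for Lerp snapping.
; Overlaps toggle a wrist cylinder highlight, which release and reset hide.
; Both cylinder meshes are destroyed on Oculus Quest and Go.
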(event `self.ReceiveBeginPlay`
  (`parent.ReceiveBeginPlay`)
  (switch `name` (`HeadMountedDisplayFunctionLibrary.GetHMDDeviceName`)
    (:`OculusHMD`
      (switch `string` (`OculusFunctionLibrary.GetDeviceName`)
        (:`Oculus Quest`
          _)
        (:`Oculus Go`
          _))
      (`ActorComponent.K2_DestroyComponent` (`self.WristCylinder`))
      (`ActorComponent.K2_DestroyComponent` (`self.WristCylinderFlipped`)))))

(event `self.ReceiveTick`
  (params (DeltaSeconds :type "Float (single-precision)"))
  (bind (_bvalid_ _returnvalue) (`self.GetInventoryComponent`))
  (bind (_bvalid__2 _returnvalue_2) (`self.GetInventoryComponent`))
  ;[1 1 1] Update the object location when the hand overlaps
  (`parent.ReceiveTick` DeltaSeconds)
  (if (`self.TrackHand`)
    (`self.ItemToStore`
      (:`then`
        (`|ExecutionSequence`
          (:`then_0`
            (switch `/Game/VRInv/Miscellaneous/ESlotSnapType` (`self.SlotSnapType`)
              (:`NewEnumerator0`
                (if _bvalid__2
                  (`/Game/VRInv/Blueprints/BPC_InventoryItem.AttachToComp` _returnvalue_2 ; Check if the item to store is valid
                    (:`then`
                      _)
                    (:`else`)))
                (`self.HandReference` ; Check if we have a valid hand ref\nif we do it means we already dropped\nthe object in the slot and want to retrieve \nit. So we play the object to hand effect\nwhich is based on the hand distance \nfrom the wrist pocket
                  (:`then`
                    (`self.K2_SetActorTransform` (`self.ItemToStore`) (`self.GetObjectTransform`) false false))
                  (:`else`)))))
          (:`then_1`
            (`SceneComponent.K2_SetWorldRotation` (`self.ItemLocation`) (`KismetMathLibrary.FindLookAtRotation` (`SceneComponent.K2_GetComponentLocation` (`self.ItemLocation`)) (`SceneComponent.GetSocketLocation` (`/Game/VRInv/Blueprints/BPC_InventoryItem.AttachToComp` _returnvalue) (`/Game/VRInv/Blueprints/BPC_InventoryItem.SocketName` _returnvalue))) false false) ; This makes the wrist pocket look at the hand
          )))
      (:`else`))
    (else
      (`self.ItemToStore` ; Here we are not tracking the hand but still\nneed to have a valid item stored reference\nthis check allows us to understand whether\nthe wrist pocket contains an object or not.
        (:`then`
          (`SceneComponent.K2_SetWorldRotation` (`self.ItemLocation`) (`KismetMathLibrary.FindLookAtRotation` (`SceneComponent.K2_GetComponentLocation` (`self.ItemLocation`)) (`PlayerCameraManager.GetCameraLocation` (`GameplayStatics.GetPlayerCameraManager` 0))) false false))
        (:`else`)))))

(event `self.OnItemReleased`
  (`parent.OnItemReleased`)
  (`self.ShowHideWristCylinder` true))

(fn `ProcessHandEndOverlap`
  (params (OtherActor :type "Actor Object Reference") (OtherComponent :type "PrimitiveComponent Object Reference"))
  (`parent.ProcessHandEndOverlap` OtherActor OtherComponent)
  (`SceneComponent.K2_SetRelativeRotation` (`self.ItemLocation`) (struct :`Pitch` 90.0) false false)
  (`self.ShowHideWristCylinder` true))

(fn `ProcessHandOverlap`
  (params (OtherActor :type "Actor Object Reference") (OtherComponent :type "PrimitiveComponent Object Reference"))
  (`parent.ProcessHandOverlap` OtherActor OtherComponent)
  (`self.ShowHideWristCylinder` false))

(fn `ProcessNewObjectOverlap`
  (params (OtherActor :type "Actor Object Reference") (OtherComponent :type "PrimitiveComponent Object Reference"))
  (`parent.ProcessNewObjectOverlap` OtherActor OtherComponent)
  (if (`self.IsObjectValidIventoryItem?` OtherActor OtherComponent)
    (`self.ShowHideWristCylinder` false)))

(fn `ResetState`
  (`parent.ResetState`)
  (`SceneComponent.K2_SetRelativeRotation` (`self.ItemLocation`) (struct :`Pitch` 90.0) false false)
  (`self.ShowHideWristCylinder` true))

(fn `ShowHideWristCylinder`
  (params (NewHidden :type Boolean))
  (`self.WristCylinder`
    (:`then`
      (`SceneComponent.SetHiddenInGame` (`self.WristCylinder`) NewHidden false))
    (:`else`)))

(fn `UserConstructionScript`
  (`parent.UserConstructionScript`))