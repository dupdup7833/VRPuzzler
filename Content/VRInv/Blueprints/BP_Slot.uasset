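; VR wrist inventory slot actor that stores a held item carrying BPC_InventoryItem when released inside its collision sphere.
; Overlaps accept items not held by the slot's own hand, then track hands near occupied slots.
; On release it disables physics, lerps or snaps the item into place at reduced scale, attaches it and swaps materials; pickup restores it.
; GetObjectTransform computes an interpolated slot-to-hand transform, blending location and scale by hand distance.
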(event `OnItemReleased`
  (bind (_bvalid_ _returnvalue) (`self.GetInventoryComponent`))
  (bind (_returnvalue_location _returnvalue_rotation) (`KismetMathLibrary.BreakTransform` (`SceneComponent.K2_GetComponentToWorld` (`self.ItemLocation`))))
  (bind (_returnvalue_location_2 _returnvalue_rotation_2) (`KismetMathLibrary.BreakTransform` (`SceneComponent.K2_GetComponentToWorld` (`self.ItemLocation`))))
  ;[1 1 1] Snap item to slot
  ;;[1 1 1] Make sure we should snap to the slot
  (if (`self.ShouldStoreItem`)
    (set `self.TrackHand` false)
    (set `self.bIsSlotUsed?` true)
    (bind _itemtostore (`self.ItemToStore`)
      (:`then`
        (if (`self.IsWristSlotOnOtherHand?` _itemtostore)
          ;;[1 1 1] Prepare for snapping. Disable physics get current actor transform and scale timeline
          (`|ExecutionSequence`
            (:`then_0`
              (if _bvalid_
                (`PrimitiveComponent.SetSimulatePhysics` (`/Game/VRInv/Blueprints/BPC_InventoryItem.GetMesh` _returnvalue) false)
                (set `/Game/VRInv/Blueprints/BPC_InventoryItem.bItemStored?` true _returnvalue)
                (`/Game/VRInv/Blueprints/BPC_InventoryItem.OnItemStored` _returnvalue)))
            (:`then_1`
              (`self.GetStoredTargetScale` :!label _label)
              (switch `/Game/VRInv/Miscellaneous/ESlotSnapType` (`self.SlotSnapType`)
                (:`NewEnumerator0`
                  ;[1 1 1] Snap to the slot by lerping
                  (set `self.ItemInitTransform` (`self.GetTransform` (`self.ItemToStore`)))
                  (`TimelineComponent.SetPlayRate` (`self.SnapToWrist`) (/ 1.0 (`self.HandToSlotAnimationDuration`)))
                  (bind (_direction _alpha) (`Timeline|SnapToWrist` :!via `PlayFromStart`)
                    (:`Update`
                      (`self.ItemToStore`
                        (:`then`
                          (`self.K2_SetActorTransform` (`self.ItemToStore`) (`KismetMathLibrary.TLerp` (`self.ItemInitTransform`) (`KismetMathLibrary.MakeTransform` _returnvalue_location _returnvalue_rotation (`self.StoredTargetScale`)) _alpha) false false))
                        (:`else`)))
                    (:`Finished`
                      (`self.K2_AttachToComponent` (`self.ItemToStore`) (`self.RootComponent`) "None" "KeepWorld" "KeepWorld" "KeepWorld" false :!label _label_2)
                      (`self.UpdateItemStoredMaterials`))))
                (:`NewEnumerator1`
                  ;[1 1 1] Snap to the slot by just setting the transform
                  (`self.ItemToStore`
                    (:`then`
                      (`self.K2_SetActorTransform` (`self.ItemToStore`) (`KismetMathLibrary.MakeTransform` _returnvalue_location_2 _returnvalue_rotation_2 (`self.StoredTargetScale`)) false false)
                      (goto _label_2))
                    (:`else`))))))))
      (:`else`))))

(event `ObjectToSlot`
  ;[1 1 1] Snap item to slot
  (goto _label))

(event `OnItemStoredPickedup`
  (bind (_bvalid_ _returnvalue) (`self.GetInventoryComponent`))
  ;[1 1 1] On Object Picked up we want to make sure that the object is being tracked and that is valid so we can reset the slot state
  (`self.ItemToStore`
    (:`then`
      (`|ExecutionSequence`
        (:`then_0`
          (if _bvalid_
            (set `/Game/VRInv/Blueprints/BPC_InventoryItem.bItemStored?` false _returnvalue)
            (`/Game/VRInv/Blueprints/BPC_InventoryItem.OnItemRetrieved` _returnvalue)))
        (:`then_1`
          (if (`self.IsActorTickEnabled`)
            (set `self.TrackHand` false)
            (`self.ResetState`)))))
    (:`else`)))

(event `self.SlotCollision.OnComponentBeginOverlap`
  (params (OverlappedComponent :type "PrimitiveComponent Object Reference") (OtherActor :type "Actor Object Reference") (OtherComp :type "PrimitiveComponent Object Reference") (OtherBodyIndex :type Integer) (bFromSweep :type Boolean) (SweepResult :type "HitResult Structure (by ref)"))
  ;[1 1 1] On slot collision events
  (if (not (`self.bIsSlotUsed?`))
    (`self.ProcessNewObjectOverlap` OtherActor OtherComp)
    (else
      (`self.ProcessHandOverlap` OtherActor OtherComp))))

(event `self.SlotCollision.OnComponentEndOverlap`
  (params (OverlappedComponent :type "PrimitiveComponent Object Reference") (OtherActor :type "Actor Object Reference") (OtherComp :type "PrimitiveComponent Object Reference") (OtherBodyIndex :type Integer))
  ;[1 1 1] On slot collision events
  (if (not (`self.bIsSlotUsed?`))
    (`self.ProcessObjectEndOverlap` OtherActor OtherComp)
    (else
      (`self.ProcessHandEndOverlap` OtherActor OtherComp))))

(fn `GetHandSlotDistAlpha`
  (returns (ReturnValue :type "Float (double-precision)"))
  (bind _sphereradius (`SphereComponent.SphereRadius` (`self.SlotCollision`)))
  (return (`KismetMathLibrary.MapRangeClamped` (`KismetMathLibrary.Abs` (`KismetMathLibrary.VSize` (- (`SceneComponent.K2_GetComponentLocation` (`self.HandReference`)) (`self.K2_GetActorLocation`)))) _sphereradius (* _sphereradius 2.0) 1.0)))

(fn `GetInventoryComponent`
  (returns (`bValid?` :type Boolean) (ReturnValue :type "/Game/VRInv/Blueprints/BPC_InventoryItem Object Reference"))
  (bind _returnvalue (`self.GetComponentByClass` (`self.ItemToStore`) "/Game/VRInv/Blueprints/BPC_InventoryItem.BPC_InventoryItem_C"))
  (`/Engine/EditorBlueprintResources/StandardMacros.IsValid` _returnvalue
    (:`Is Valid`
      (return true _returnvalue))
    (:`Is Not Valid`
      (return false null))))

(fn `GetObjectTransform`
  (returns (ReturnValue :type "Transform Structure"))
  (bind (_bvalid_ _returnvalue) (`self.GetInventoryComponent`))
  (bind (_bvalid__2 _returnvalue_2) (`self.GetInventoryComponent`))
  (bind (_returnvalue_location _returnvalue_rotation) (`KismetMathLibrary.BreakTransform` (`SceneComponent.K2_GetComponentToWorld` (`/Game/VRInv/Blueprints/BPC_InventoryItem.AttachToComp` (`.ReturnValue` (`self.GetInventoryComponent`))))))
  (bind _returnvalue_location_2 (`KismetMathLibrary.BreakTransform` (`SceneComponent.K2_GetComponentToWorld` (`/Game/VRInv/Blueprints/BPC_InventoryItem.AttachToComp` (`.ReturnValue` (`self.GetInventoryComponent`))))))
  (return (`KismetMathLibrary.TInterpTo` (`self.GetTransform` (`self.ItemToStore`)) (`KismetMathLibrary.MakeTransform` (`KismetMathLibrary.VLerp` (`SceneComponent.K2_GetComponentLocation` (`self.ItemLocation`)) (`KismetMathLibrary.SelectVector` (`SceneComponent.GetSocketLocation` (`/Game/VRInv/Blueprints/BPC_InventoryItem.AttachToComp` _returnvalue) (`/Game/VRInv/Blueprints/BPC_InventoryItem.SocketName` _returnvalue)) _returnvalue_location_2 (`/Game/VRInv/Blueprints/BPC_InventoryItem.bSnapToSocket?` _returnvalue)) (`self.GetHandSlotDistAlpha`)) (`KismetMathLibrary.SelectRotator` (`SceneComponent.GetSocketRotation` (`/Game/VRInv/Blueprints/BPC_InventoryItem.AttachToComp` _returnvalue_2) (`/Game/VRInv/Blueprints/BPC_InventoryItem.SocketName` _returnvalue_2)) _returnvalue_rotation (`/Game/VRInv/Blueprints/BPC_InventoryItem.bSnapToSocket?` _returnvalue_2)) (`KismetMathLibrary.VLerp` (`self.StoredTargetScale`) (`/Game/VRInv/Blueprints/BPC_InventoryItem.InitialScale` (`.ReturnValue` (`self.GetInventoryComponent`))) (`self.GetHandSlotDistAlpha`))) (`GameplayStatics.GetWorldDeltaSeconds`) (`self.ObjectToHandAnimInterSpeed`))))

(fn `GetStoredTargetScale`
  (bind (_bvalid_ _returnvalue) (`self.GetInventoryComponent`))
  (`self.ItemToStore`
    (:`then`
      (`/Engine/EditorBlueprintResources/StandardMacros.IsValid` _returnvalue
        (:`Is Valid`
          (set `self.StoredTargetScale` (* (`/Game/VRInv/Blueprints/BPC_InventoryItem.InitialScale` _returnvalue) (/ (`/Game/VRInv/Blueprints/BPC_InventoryItem.WristStoredScalePercentage` _returnvalue) 100.0)))
          (return))))
    (:`else`)))

(fn `IsObjectValidIventoryItem?`
  (params (OtherActor :type "Actor Object Reference") (OtherComponent :type "SceneComponent Object Reference"))
  (returns (ReturnValue :type Boolean))
  (bind _returnvalue (`self.GetComponentByClass` (`local.OtherActor`) "/Game/VRInv/Blueprints/BPC_InventoryItem.BPC_InventoryItem_C"))
  (`/Engine/EditorBlueprintResources/StandardMacros.IsValid` _returnvalue
    (:`Is Valid`
      (if (`KismetSystemLibrary.DoesImplementInterface` (`local.OtherActor`) "/Game/VRInv/Blueprints/BI_GrabForcePickup.BI_GrabForcePickup_C")
        (bind _result (message `/Game/VRInv/Blueprints/BI_GrabForcePickup.Held?` (`local.OtherActor`)))
        (return (and _result (== (`/Game/VRInv/Blueprints/BPC_InventoryItem.GetMesh` _returnvalue) (`local.OtherComponent`)) (`/Game/VRInv/Blueprints/BPC_InventoryItem.bCanBeStored?` _returnvalue)))
        (else
          (return false))))
    (:`Is Not Valid`
      (return false))))

(fn `IsWristSlotOnOtherHand?`
  (params (Item :type "Actor Object Reference"))
  (returns (ReturnValue :type Boolean))
  (bind _returnvalue (`self.GetComponentByClass` Item "/Game/VRInv/Blueprints/BPC_InventoryItem.BPC_InventoryItem_C"))
  (bind _attachtocomp (`/Game/VRInv/Blueprints/BPC_InventoryItem.AttachToComp` _returnvalue))
  (bind _result (message `/Game/VRInv/Blueprints/BI_GrabForcePickup.Held?` Item))
  (`/Engine/EditorBlueprintResources/StandardMacros.IsValid` _returnvalue
    (:`Is Valid`
      (`/Engine/EditorBlueprintResources/StandardMacros.IsValid` _attachtocomp
        (:`Is Valid`
          (bind _returnvalue_2 (and _result (and (!= (`ActorComponent.GetOwner` _attachtocomp) (`self.GetParentActor`)) (!= _attachtocomp (`self.GetParentComponent`)))))
          (if _returnvalue_2
            (return _returnvalue_2)
            (else
              (return (`|EnumInequality` (`/Game/VRInv/Blueprints/BPC_InventoryItem.Hand` _returnvalue) (`self.Hand`))))))
        (:`Is Not Valid`
          (return false))))
    (:`Is Not Valid`
      (return false))))

(fn `ProcessHandEndOverlap`
  (params (OtherActor :type "Actor Object Reference") (OtherComponent :type "PrimitiveComponent Object Reference"))
  (bind (_bvalid_ _returnvalue) (`self.GetInventoryComponent`))
  (if (or (`ActorComponent.ComponentHasTag` OtherComponent "InventoryInteraction") (`ActorComponent.ComponentHasTag` OtherComponent "inventoryinteraction"))
    (if (`self.TrackHand`)
      (set `self.TrackHand` false)
      (`self.ObjectToSlot`)
      (if _bvalid_
        (set `/Game/VRInv/Blueprints/BPC_InventoryItem.bCanPickupItem?` false _returnvalue)))))

(fn `ProcessHandOverlap`
  (params (OtherActor :type "Actor Object Reference") (OtherComponent :type "PrimitiveComponent Object Reference"))
  (bind (_bvalid_ _returnvalue) (`self.GetInventoryComponent`))
  (if (or (`ActorComponent.ComponentHasTag` OtherComponent "InventoryInteraction") (`ActorComponent.ComponentHasTag` OtherComponent "inventoryinteraction"))
    (set `self.HandReference` OtherComponent)
    (set `self.TrackHand` true)
    (if _bvalid_
      (set `/Game/VRInv/Blueprints/BPC_InventoryItem.bCanPickupItem?` true _returnvalue))))

(fn `ProcessNewObjectOverlap`
  (params (OtherActor :type "Actor Object Reference") (OtherComponent :type "PrimitiveComponent Object Reference"))
  (bind (_bvalid_ _returnvalue) (`self.GetInventoryComponent`))
  (bind _returnvalue_2 (`self.GetComponentByClass` (`self.ItemToStore`) "/Game/VRInv/Blueprints/BPC_InventoryItem.BPC_InventoryItem_C"))
  (if (`self.IsObjectValidIventoryItem?` OtherActor OtherComponent)
    (if (`self.IsWristSlotOnOtherHand?` (`local.OtherActor`))
      (set `self.ItemToStore` (`local.OtherActor`))
      (`|ExecutionSequence`
        (:`then_0`
          (`/Engine/EditorBlueprintResources/StandardMacros.IsValid` _returnvalue_2
            (:`Is Valid`
              (add `/Game/VRInv/Blueprints/BPC_InventoryItem.OnPickup` _returnvalue_2 (`|CreateDelegate` :!event `OnItemStoredPickedup`))
              (add `/Game/VRInv/Blueprints/BPC_InventoryItem.OnRelease` _returnvalue_2 (`|CreateDelegate` :!event `OnItemReleased`)))))
        (:`then_1`
          (set `self.ShouldStoreItem` true)
          (set `self.TrackHand` true)
          (`self.UpdateItemCollision` false)
          (if _bvalid_
            (set `/Game/VRInv/Blueprints/BPC_InventoryItem.bCanPickupItem?` false _returnvalue))))
      (else
        (set `self.ShouldStoreItem` false)))))

(fn `ProcessObjectEndOverlap`
  (params (OtherActor :type "Actor Object Reference") (OtherComponent :type "PrimitiveComponent Object Reference"))
  (bind _returnvalue (`self.GetComponentByClass` OtherActor "/Game/VRInv/Blueprints/BPC_InventoryItem.BPC_InventoryItem_C"))
  (`/Engine/EditorBlueprintResources/StandardMacros.IsValid` _returnvalue
    (:`Is Valid`
      (if (`KismetSystemLibrary.DoesImplementInterface` OtherActor "/Game/VRInv/Blueprints/BI_GrabForcePickup.BI_GrabForcePickup_C")
        (bind _result (message `/Game/VRInv/Blueprints/BI_GrabForcePickup.Held?` OtherActor))
        (if (and _result (== (`/Game/VRInv/Blueprints/BPC_InventoryItem.GetMesh` _returnvalue) (`local.OtherComponent`)))
          (`self.ItemToStore`
            (:`then`
              (set `self.TrackHand` false)
              (`self.ResetState`))
            (:`else`)))))))

(fn `ResetState`
  (bind (_bvalid_ _returnvalue) (`self.GetInventoryComponent`))
  (bind (_bvalid__2 _returnvalue_2) (`self.GetInventoryComponent`))
  (bind _returnvalue_3 (`self.GetComponentByClass` (`self.ItemToStore`) "/Game/VRInv/Blueprints/BPC_InventoryItem.BPC_InventoryItem_C"))
  (set `self.bIsSlotUsed?` false)
  (set `self.ShouldStoreItem` false)
  (`|ExecutionSequence`
    (:`then_0`
      (if _bvalid_
        (set `/Game/VRInv/Blueprints/BPC_InventoryItem.bCanPickupItem?` true _returnvalue)))
    (:`then_1`
      (`/Engine/EditorBlueprintResources/StandardMacros.IsValid` _returnvalue_3
        (:`Is Valid`
          (add `/Game/VRInv/Blueprints/BPC_InventoryItem.OnPickup` _returnvalue_3 (`|CreateDelegate` :!event `OnItemStoredPickedup`))
          (add `/Game/VRInv/Blueprints/BPC_InventoryItem.OnRelease` _returnvalue_3 (`|CreateDelegate` :!event `OnItemReleased`)))))
    (:`then_2`
      (`self.SetActorScale3D` (`self.ItemToStore`) (`/Game/VRInv/Blueprints/BPC_InventoryItem.InitialScale` (`.ReturnValue` (`self.GetInventoryComponent`))))
      (for (_ _array_index) (`MeshComponent.GetMaterials` (`/Game/VRInv/Blueprints/BPC_InventoryItem.GetMesh` (`.ReturnValue` (`self.GetInventoryComponent`))))
        (`PrimitiveComponent.SetMaterial` (`/Game/VRInv/Blueprints/BPC_InventoryItem.GetMesh` _returnvalue_2) _array_index (`|GetArrayItem` (`/Game/VRInv/Blueprints/BPC_InventoryItem.DefaultMaterials` _returnvalue_2) _array_index)))
      (`self.UpdateItemCollision` true)
      (set `self.ItemToStore` null)
      (set `self.HandReference` null))))

(fn `UpdateItemCollision`
  (params (CollisionEnabled :type Boolean))
  (locals (CachedItemLocation :type "Actor Object Reference"))
  (bind _mesh (`/Game/VRInv/Blueprints/BPC_InventoryItem.GetMesh` (`.ReturnValue` (`self.GetInventoryComponent`))))
  (bind _itemtostore (`self.ItemToStore`)
    (:`then`
      (set `local.CachedItemLocation` _itemtostore)
      (if (`local.CollisionEnabled`)
        (`PrimitiveComponent.SetCollisionEnabled` (`/Game/VRInv/Blueprints/BPC_InventoryItem.GetMesh` (`.ReturnValue` (`self.GetInventoryComponent`))) (`self.ItemStoredCollision`))
        (else
          (set `self.ItemStoredCollision` (`PrimitiveComponent.GetCollisionEnabled` _mesh))
          (`PrimitiveComponent.SetCollisionEnabled` _mesh "QueryOnly")))
      (set `self.ItemToStore` (`local.CachedItemLocation`))
      (return))
    (:`else`)))

(fn `UpdateItemStoredMaterials`
  (bind _mesh (`/Game/VRInv/Blueprints/BPC_InventoryItem.GetMesh` (`.ReturnValue` (`self.GetInventoryComponent`))))
  (for (_ _array_index) (`MeshComponent.GetMaterials` _mesh)
    (`PrimitiveComponent.SetMaterial` _mesh _array_index (`self.ItemStoredMaterial`))))

(fn `UserConstructionScript`)